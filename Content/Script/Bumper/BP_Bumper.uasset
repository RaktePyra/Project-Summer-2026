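; Bumper actor that bounces the player and objects entering its Sphere, unless it is stickied.
; BP_FirstPersonCharacter is launched with its overlapping component's velocity, vertically inverted.
; Other overlaps apply a velocity-change impulse to both components, using a reflection-like direction (cross rather than dot product) scaled by speed and BouncyFactorForObjects.
; Sticky and UnSticky events toggle bouncing, with debug prints throughout.
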(event OnComponentBeginOverlap(Sphere)
  (params (OverlappedComponent :type Primitive%20Component%20Object%20Reference) (OtherActor :type Actor%20Object%20Reference) (OtherComp :type Primitive%20Component%20Object%20Reference) (OtherBodyIndex :type Integer) (bFromSweep :type Boolean) (SweepResult :type Hit%20Result%20Structure%20%28by%20ref%29))
  (bind _returnvalue (Transformation|GetComponentVelocity OtherComp))
  (bind _returnvalue_2 (Transformation|GetComponentVelocity OtherComp))
  (bind _sphere (Variables|Default|GetSphere))
  (bind (_x _y _z) (Math|Vector|BreakVector _returnvalue))
  (bind _returnvalue_3 (Math|Vector|GetUpVector _sphere))
  (bind _returnvalue_4 (Math|Vector|Normalize _returnvalue_2))
  (bind _returnvalue_5 (Math|Vector|CrossProduct _returnvalue_3 _returnvalue_4))
  (bind _returnvalue_6 (* _returnvalue_5 _returnvalue_3))
  (bind _returnvalue_7 (* _returnvalue_6 2.0))
  (bind _returnvalue_8 (- _returnvalue_2 _returnvalue_7))
  (if (not (Variables|Default|GetIsStickied))
    (bind _asbp_first_person_character (Utilities|Casting|CastToBP_FirstPersonCharacter OtherActor)
      (:then
        (Character|LaunchCharacter _asbp_first_person_character (Math|Vector|MakeVector _x _y (* _z -1.0)) true true)
        (Development|PrintString (Utilities|String|Append "Initial VELOCITY :" (Utilities|String|ToString(Vector) _returnvalue))))
      (:CastFailed
        (Physics|AddImpulse OverlappedComponent (* (* (Math|Vector|Normalize _returnvalue_8) (Math|Vector|VectorLength _returnvalue_2)) (Variables|Default|GetBouncyFactor%20for%20objects)) "None" true)
        (Development|PrintString (Utilities|String|ToString(Vector) _returnvalue_8))))))

(event EventBeginPlay)

(event Collision|EventActorBeginOverlap
  (params (OtherActor :type Actor%20Object%20Reference)))

(event EventTick
  (params (DeltaSeconds :type Float%20%28single-precision%29)))

(event EventSticky
  (Variables|Default|SetIsStickied true)
  (Development|PrintString "Bumper : Stickied"))

(event EventUnSticky
  (Variables|Default|SetIsStickied false)
  (Development|PrintString "Bumper : Unstickied"))

(fn ConstructionScript)