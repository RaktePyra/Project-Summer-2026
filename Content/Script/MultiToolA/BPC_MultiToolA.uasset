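; First-person multi-tool weapon component that repulses objects and fires sticky splash projectiles.
; On BeginPlay it attaches to the character's GripPoint, adds the weapon input mapping and sets the rifle animation flag.
; Shoot either box-traces filtered to a cone or, while ongoing, sphere-traces a ray, by configuration, calling IRepulsable or applying impulses.
; Projectiles spawn from the Ammo socket with a gun back-reference, and accessors store the active sticky surface.
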(event Input|EnhancedActionEvents|EnhancedInputActionIA_Shoot
  (params (ActionValue :type Boolean) (ElapsedSeconds :type Float%20%28double-precision%29) (TriggeredSeconds :type Float%20%28double-precision%29) (InputAction :type Input%20Action%20Object%20Reference :default "/Game/FirstPerson/Input/Actions/IA_Shoot.IA_Shoot"))
  (bind _ownergameobject (Variables|Default|GetOwnerGameObject))
  (bind _ownergameobject_2 (Variables|Default|GetOwnerGameObject))
  (bind _box_radius_for_impulse_detection_a (Variables|ConfigA|GetBox%20Radius%20for%20Impulse%20Detection%20A))
  (bind _ownergameobject_3 (Variables|Default|GetOwnerGameObject))
  (bind _cone_angle_a (Variables|ConfigA|GetCone%20Angle%20A))
  (bind _returnvalue (Transformation|GetActorLocation _ownergameobject))
  (bind _returnvalue_2 (Actor|GetComponentbyClass _ownergameobject_2 "/Script/Engine.CameraComponent"))
  (bind _returnvalue_3 (Actor|GetComponentbyClass _ownergameobject_3 "/Script/Engine.CameraComponent"))
  (:Triggered
    (if (Variables|Default|GetIsConfigurationA)
      (Utilities|IsValid _returnvalue_3
        (:Is%20Valid
          (Variables|Default|SetRotationToUseForTrace (Transformation|GetWorldRotation _returnvalue_3)))
        (:Is%20Not%20Valid
          (Variables|Default|SetRotationToUseForTrace (Transformation|GetActorRotation (Variables|Default|GetOwnerGameObject)))))
      (bind _outhits (Class|KismetSystemLibrary|BoxTraceMulti (+ (Transformation|GetActorLocation (Variables|Default|GetOwnerGameObject)) (Math|Vector|RotateVector (Math|Vector|MakeVector (Variables|ConfigA|GetBox%20Radius%20for%20Impulse%20Detection%20A) 0.0 0.0) (Variables|Default|GetRotationToUseForTrace))) (+ (Transformation|GetActorLocation (Variables|Default|GetOwnerGameObject)) (Math|Vector|RotateVector (Math|Vector|MakeVector (Variables|ConfigA|GetBox%20Radius%20for%20Impulse%20Detection%20A) 0.0 0.0) (Variables|Default|GetRotationToUseForTrace))) (Math|Vector|MakeVector _box_radius_for_impulse_detection_a _box_radius_for_impulse_detection_a _box_radius_for_impulse_detection_a) (Variables|Default|GetRotationToUseForTrace) "TraceTypeQuery1" false 0 "ForDuration" true))
      (for _array_element _outhits
        (Variables|Default|SetHit%20Actor%20A (.HitActor (Collision|BreakHitResult _array_element)))
        (if (and (<= (Class|KismetMathLibrary|DegAcos (Math|Vector|DotProduct (* (Math|Vector|Normalize (- (Transformation|GetActorLocation (Variables|Default|GetHit%20Actor%20A)) (Transformation|GetActorLocation (Variables|Default|GetOwnerGameObject)))) (Variables|ConfigA|GetImpulsion%20Intensity%20A)) (Math|Rotator|GetRotationXVector (Variables|Default|GetRotationToUseForTrace)))) _cone_angle_a) (>= (Class|KismetMathLibrary|DegAcos (Math|Vector|DotProduct (* (Math|Vector|Normalize (- (Transformation|GetActorLocation (Variables|Default|GetHit%20Actor%20A)) (Transformation|GetActorLocation (Variables|Default|GetOwnerGameObject)))) (Variables|ConfigA|GetImpulsion%20Intensity%20A)) (Math|Rotator|GetRotationXVector (Variables|Default|GetRotationToUseForTrace)))) (* _cone_angle_a -1.0)))
          (if (<= (Math|Vector|VectorLength (- (.Location (Collision|BreakHitResult _array_element)) (Transformation|GetActorLocation (Variables|Default|GetOwnerGameObject)))) (Variables|ConfigA|GetCone%20Radius))
            (if (Utilities|DoesObjectImplementInterface (Variables|Default|GetHit%20Actor%20A) "/Game/Script/MultiToolA/IRepulsable.IRepulsable_C")
              (Class|IRepulsable|Repulse(Message) (Variables|Default|GetHit%20Actor%20A))
              (elif (Physics|IsSimulatingPhysics (Variables|/Script/Engine.Actor|GetRootComponent (Variables|Default|GetHit%20Actor%20A)) "None")
                (bind _asprimitive_component (Utilities|Casting|CastToPrimitiveComponent (Variables|/Script/Engine.Actor|GetRootComponent (Variables|Default|GetHit%20Actor%20A))))
                (Physics|AddImpulse _asprimitive_component (* (* (Math|Vector|Normalize (- (Transformation|GetActorLocation (Variables|Default|GetHit%20Actor%20A)) (Transformation|GetActorLocation (Variables|Default|GetOwnerGameObject)))) (Variables|ConfigA|GetImpulsion%20Intensity%20A)) 1e+05) "None" false)
                (Development|PrintString "Impulse"))))))))
  (:Ongoing
    (if (not (Variables|Default|GetIsConfigurationA))
      (Utilities|IsValid _returnvalue_2
        (:Is%20Valid
          (Variables|Default|SetRotationToUseForTrace (Transformation|GetWorldRotation _returnvalue_2)))
        (:Is%20Not%20Valid
          (Variables|Default|SetRotationToUseForTrace (Transformation|GetActorRotation (Variables|Default|GetOwnerGameObject)))))
      (bind _outhit (Collision|SphereTraceByChannel _returnvalue (+ _returnvalue (* (Math|Vector|GetForwardVector _returnvalue_2) (Variables|ConfigB|GetRayLength))) (Variables|ConfigB|GetRayRadiusB) "TraceTypeQuery1" false 0 "ForDuration"))
      (bind _output_get (Variables|Default|SetHit%20Actor%20B (.hitactor _outhit)))
      (Utilities|IsValid _output_get
        (:Is%20Valid
          (if (Utilities|DoesObjectImplementInterface _output_get "/Game/Script/MultiToolA/IRepulsable.IRepulsable_C")
            (Class|IRepulsable|Repulse(Message) (Variables|Default|GetHit%20Actor%20B))
            (else
              (Utilities|IsValid (Variables|/Script/Engine.Actor|GetRootComponent (Variables|Default|GetHit%20Actor%20B))
                (:Is%20Valid
                  (bind _asprimitive_component_2 (Utilities|Casting|CastToPrimitiveComponent (Variables|/Script/Engine.Actor|GetRootComponent (Variables|Default|GetHit%20Actor%20B))))
                  (Physics|AddImpulse _asprimitive_component_2 (* (* (Math|Vector|Normalize (- (Transformation|GetActorLocation (Variables|Default|GetHit%20Actor%20B)) (Transformation|GetActorLocation (Variables|Default|GetOwnerGameObject)))) (Variables|ConfigB|GetImpulsion%20Intensity%20B)) 1e+05) "None" false))))))))))

(event Input|EnhancedActionEvents|EnhancedInputActionIA_StickySplash
  (params (ActionValue :type Boolean) (ElapsedSeconds :type Float%20%28double-precision%29) (TriggeredSeconds :type Float%20%28double-precision%29) (InputAction :type Input%20Action%20Object%20Reference :default "/Game/FirstPerson/Input/Actions/IA_StickySplash.IA_StickySplash"))
  (bind _returnvalue (Game|GetPlayerCameraManager 0))
  (bind _returnvalue_2 (Transformation|GetSocketLocation "Ammo"))
  (bind _projectile_offset (Variables|Default|GetProjectile%20Offset))
  (bind _returnvalue_3 (Camera|GetCameraRotation _returnvalue))
  (bind _returnvalue_4 (Math|Vector|RotateVector _projectile_offset _returnvalue_3))
  (bind _returnvalue_5 (+ _returnvalue_2 _returnvalue_4))
  (bind _returnvalue_6 (Game|SpawnActorfromClass "/Game/Script/MultiToolA/BP_StickySplashProjectile.BP_StickySplashProjectile_C" (Math|Transform|MakeTransform _returnvalue_5 _returnvalue_3) "Undefined" "OverrideRootScale" 0 0))
  (Variables|/Game/Script/MultiToolA/BP_StickySplashProjectile.BP_StickySplashProjectile_C|SetGunOrigin _returnvalue_6 self)
  (Audio|PlaySoundatLocation "/Game/FPWeapon/Audio/FirstPersonTemplateWeaponFire02.FirstPersonTemplateWeaponFire02" _returnvalue_5 "0, 0, 0" 1.0 1.0 0.0 0 0 0 0) ; Play firing sound
)

(event EventBeginPlay
  (bind _returnvalue (Components|GetOwner))
  (Variables|Default|SetOwnerGameObject _returnvalue)
  (bind _asbp_first_person_character (Utilities|Casting|CastToBP_FirstPersonCharacter _returnvalue))
  (Variables|Default|SetAs%20BP%20First%20Person%20Character _asbp_first_person_character)
  (Transformation|AttachComponentToComponent (Variables|/Game/FirstPerson/Blueprints/BP_FirstPersonCharacter.BP_FirstPersonCharacter_C|GetFirstPersonMesh _asbp_first_person_character) "GripPoint" "SnapToTarget" "SnapToTarget" "SnapToTarget" true)
  (bind _asplayer_controller (Utilities|Casting|CastToPlayerController (Pawn|GetController (Variables|Default|GetAs%20BP%20First%20Person%20Character))))
  (Utilities|IsValid (PlayerController|LocalPlayerSubsystems|GetEnhancedInputLocalPlayerSubsystem _asplayer_controller)
    (:Is%20Valid
      (Input|AddMappingContext (PlayerController|LocalPlayerSubsystems|GetEnhancedInputLocalPlayerSubsystem _asplayer_controller) "/Game/FirstPerson/Input/IMC_Weapons.IMC_Weapons" 0 "(bIgnoreAllPressedKeysUntilRelease=True,bForceImmediately=False,bNotifyUserSettings=False)")
      (bind _asfirst_person_anim_bp (Utilities|Casting|CastToFirstPerson_AnimBP (Components|SkeletalMesh|GetAnimInstance (Variables|/Game/FirstPerson/Blueprints/BP_FirstPersonCharacter.BP_FirstPersonCharacter_C|GetFirstPersonMesh (Variables|Default|GetAs%20BP%20First%20Person%20Character)))))
      (Variables|/Game/FirstPersonArms/Animations/FirstPerson_AnimBP.FirstPerson_AnimBP_C|SetHasRifle _asfirst_person_anim_bp true))))

(event EventTick
  (params (DeltaSeconds :type Float%20%28single-precision%29)))

(fn SetActiveStickyPlatform
  (params (NewParam :type BP%20Sticky%20Surface%20Object%20Reference))
  (Variables|Default|SetActive%20Sticky%20Surface NewParam))

(fn GetActiveStickySurface
  (return (Variables|Default|GetActive%20Sticky%20Surface)))