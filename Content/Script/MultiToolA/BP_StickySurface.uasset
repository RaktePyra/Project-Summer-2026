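; Sticky surface actor that holds physics objects and characters in place while they overlap its box.
; On begin overlap it disables gravity and physics on the root primitive, zeroes character movement forces, velocity and gravity scale, and removes the first-person player's default input mapping context.
; End overlap re-enables gravity and physics without saving prior state, resets gravity scale and re-adds the mapping context.
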(event OnComponentBeginOverlap(Box)
  (params (OverlappedComponent :type Primitive%20Component%20Object%20Reference) (OtherActor :type Actor%20Object%20Reference) (OtherComp :type Primitive%20Component%20Object%20Reference) (OtherBodyIndex :type Integer) (bFromSweep :type Boolean) (SweepResult :type Hit%20Result%20Structure%20%28by%20ref%29))
  (bind _returnvalue (Actor|GetComponentbyClass OtherActor "/Script/Engine.CharacterMovementComponent"))
  (Utilities|FlowControl|Sequence
    (:then_0
      (bind _asprimitive_component (Utilities|Casting|CastToPrimitiveComponent (Variables|/Script/Engine.Actor|GetRootComponent OtherActor)))
      (Physics|SetEnableGravity _asprimitive_component false)
      (if (Physics|IsSimulatingPhysics _asprimitive_component "None")
        (Physics|SetSimulatePhysics _asprimitive_component false)))
    (:then_1
      (Utilities|IsValid _returnvalue
        (:Is%20Valid
          (Pawn|Components|CharacterMovement|ClearAccumulatedForces _returnvalue)
          (Variables|/Script/Engine.CharacterMovementComponent|SetGravityScale _returnvalue 0.0)
          (Variables|/Script/Engine.MovementComponent|SetVelocity _returnvalue "0, 0, 0"))))
    (:then_2
      (bind _asbp_first_person_character (Utilities|Casting|CastToBP_FirstPersonCharacter OtherActor))
      (Variables|Default|SetAs%20BP%20First%20Person%20Character _asbp_first_person_character)
      (bind _asplayer_controller (Utilities|Casting|CastToPlayerController (Pawn|GetController _asbp_first_person_character)))
      (bind _output_get (Variables|Default|SetAs%20Player%20Controller _asplayer_controller))
      (Utilities|IsValid (PlayerController|LocalPlayerSubsystems|GetEnhancedInputLocalPlayerSubsystem _output_get)
        (:Is%20Valid
          (Input|RemoveMappingContext (PlayerController|LocalPlayerSubsystems|GetEnhancedInputLocalPlayerSubsystem _output_get) "/Game/FirstPerson/Input/IMC_Default.IMC_Default" "(bIgnoreAllPressedKeysUntilRelease=True,bForceImmediately=False,bNotifyUserSettings=False)"))))))

(event OnComponentEndOverlap(Box)
  (params (OverlappedComponent :type Primitive%20Component%20Object%20Reference) (OtherActor :type Actor%20Object%20Reference) (OtherComp :type Primitive%20Component%20Object%20Reference) (OtherBodyIndex :type Integer))
  (bind _returnvalue (Actor|GetComponentbyClass OtherActor "/Script/Engine.CharacterMovementComponent"))
  (Utilities|FlowControl|Sequence
    (:then_0
      (bind _asprimitive_component (Utilities|Casting|CastToPrimitiveComponent (Variables|/Script/Engine.Actor|GetRootComponent OtherActor)))
      (Physics|SetEnableGravity _asprimitive_component true)
      (if (not (Physics|IsSimulatingPhysics _asprimitive_component "None"))
        (Physics|SetSimulatePhysics _asprimitive_component true)))
    (:then_1
      (Utilities|IsValid _returnvalue
        (:Is%20Valid
          (Variables|/Script/Engine.CharacterMovementComponent|SetGravityScale _returnvalue 1.0))))
    (:then_2
      (bind _asbp_first_person_character (Utilities|Casting|CastToBP_FirstPersonCharacter OtherActor))
      (Variables|Default|SetAs%20BP%20First%20Person%20Character _asbp_first_person_character)
      (bind _asplayer_controller (Utilities|Casting|CastToPlayerController (Pawn|GetController _asbp_first_person_character)))
      (bind _output_get (Variables|Default|SetAs%20Player%20Controller _asplayer_controller))
      (Utilities|IsValid (PlayerController|LocalPlayerSubsystems|GetEnhancedInputLocalPlayerSubsystem _output_get)
        (:Is%20Valid
          (Input|AddMappingContext (PlayerController|LocalPlayerSubsystems|GetEnhancedInputLocalPlayerSubsystem _output_get) "/Game/FirstPerson/Input/IMC_Default.IMC_Default" 0 "(bIgnoreAllPressedKeysUntilRelease=True,bForceImmediately=False,bNotifyUserSettings=False)"))))))

(event EventBeginPlay)

(event EventTick
  (params (DeltaSeconds :type Float%20%28single-precision%29)))

(fn ConstructionScript)