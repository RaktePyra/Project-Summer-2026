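; Projectile for a multitool gun that leaves a sticky surface where it hits, keeping one active surface per gun.
; On hit, it destroys the surface tracked by GunOrigin, spawns a BP_StickySurface at the impact point and registers it back on GunOrigin.
; The new surface's orientation derives from the hit normal rotated 90 degrees, and the projectile then destroys itself.
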(event EventBeginPlay)

(event Collision|EventActorBeginOverlap
  (params (OtherActor :type Actor%20Object%20Reference)))

(event EventTick
  (params (DeltaSeconds :type Float%20%28single-precision%29)))

(event Collision|EventHit
  (params (MyComp :type Primitive%20Component%20Object%20Reference) (Other :type Actor%20Object%20Reference) (OtherComp :type Primitive%20Component%20Object%20Reference) (bSelfMoved :type Boolean) (HitLocation :type Vector :default "0, 0, 0") (HitNormal :type Vector :default "0, 0, 0") (NormalImpulse :type Vector :default "0, 0, 0") (Hit :type Hit%20Result%20Structure%20%28by%20ref%29))
  (bind _active_sticky_surface (Default|GetActiveStickySurface (Variables|Default|GetGunOrigin)))
  (if (Utilities|IsValid _active_sticky_surface)
    (Actor|DestroyActor _active_sticky_surface))
  (bind _returnvalue (Game|SpawnActorfromClass "/Game/Script/MultiToolA/BP_StickySurface.BP_StickySurface_C" (Math|Transform|MakeTransform HitLocation (Math|Conversions|RotationFromXVector (Math|Vector|RotateVector (.normal Hit) "90.000000,0.000000,0.000000"))) "Undefined" "MultiplyWithRoot" 0 0))
  (Variables|/Game/Script/MultiToolA/BPC_MultiToolA.BPC_MultiToolA_C|SetActive%20Sticky%20Surface (Variables|Default|GetGunOrigin) _returnvalue)
  (Actor|DestroyActor))

(fn ConstructionScript)