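; BP_QTEDischargeManager is a singleton actor that starts the discharge quick-time event.
; On BeginPlay it destroys itself if GetActorOfClass returns a different instance.
; Otherwise it locks player look input, shows a WBP_QTEDischarge gauge widget with a completion time, and adds the IMC_DischargeQTE Enhanced Input mapping context.
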(event EventBeginPlay
  ;[1 0 0 0.5] Only One Instance Of this Blueprint Can Exist
  (bind _returnvalue (Actor|GetActorOfClass "BP_QTEDischargeManager_C"))
  (if (!= _returnvalue self)
    (Actor|DestroyActor self)
    (else
      (Input|SetIgnoreLookInput (Game|GetPlayerController 0) true)
      (bind _returnvalue_2 (UserInterface|CreateWidget "/Game/Script/Discharge/WBP_QTEDischarge.WBP_QTEDischarge_C"))
      (UserInterface|Viewport|AddtoViewport _returnvalue_2 0)
      (Input|AddMappingContext (PlayerController|LocalPlayerSubsystems|GetEnhancedInputLocalPlayerSubsystem) "/Game/FirstPerson/Input/Actions/DischargeQTE/IMC_DischargeQTE.IMC_DischargeQTE" 0 "(bIgnoreAllPressedKeysUntilRelease=True,bForceImmediately=False,bNotifyUserSettings=False)"))))

(fn ConstructionScript)