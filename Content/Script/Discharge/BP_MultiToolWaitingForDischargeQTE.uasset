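; Actor for a multi-tool waiting for the discharge QTE, configured as either Multi Tool A or B.
; On BeginPlay it destroys the unused tool's component and sub-battery meshes, empties the active battery fill and sets that tool's discharge state to searching.
; It also moves ForwardAxe to the active tool's location.
; UpdateSubBatteryFillAmount shows charge by setting the fill mesh's Z scale.
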(event EventBeginPlay
  (Utilities|FlowControl|Sequence
    (:then_0
      ;[0 0 1 0.5] Check if Multi Tool A or B Should Be Activate
      (switch Utilities|FlowControl|Switch|SwitchonE_MultiToolType (Variables|Components|GetActiveMultiTool)
        (:NewEnumerator0
          (Components|DestroyComponent (Variables|Default|GetBPC_MultiToolB))
          (Variables|/Game/Script/MultiTools/MultiToolA/BPC_MultiToolA.BPC_MultiToolA_C|SetIsConfigurationA (Variables|Default|GetBPC_MultiToolA) true)
          ;[0 1 1 0.5] Set Sub Battery Fil Part Z Scale to 0
          (Transformation|SetRelativeScale3D (Variables|Default|GetFBX_SubBattery_FillPart_MultiToolA) "1.000000,1.000000,0.000000")
          ;[1 0 0 0.5] Set Multi Tool In SearchingAMultiTool State
          (Variables|/Game/Script/MultiTools/MultiToolA/BPC_MultiToolA.BPC_MultiToolA_C|SetDischargeState (Variables|Default|GetBPC_MultiToolA) "NewEnumerator1"))
        (:NewEnumerator1
          (Components|DestroyComponent (Variables|Default|GetBPC_MultiToolA))
          (Transformation|SetRelativeScale3D (Variables|Default|GetFBX_SubBattery_FillPart_MultiToolB) "1.000000,1.000000,0.000000")
          (Variables|/Game/Script/MultiTools/MultiToolB/BPC_MultiToolB.BPC_MultiToolB_C|SetDischargeState (Variables|Default|GetBPC_MultiToolB) "NewEnumerator1"))))
    (:then_1
      ;[1 0 1 0.5] Set ForwardAxe At The Same World Location As The Multi Tool
      (switch Utilities|FlowControl|Switch|SwitchonE_MultiToolType (Variables|Components|GetActiveMultiTool)
        (:NewEnumerator0
          (Transformation|SetWorldLocation (Variables|Default|GetForwardAxe) (Transformation|GetWorldLocation (Variables|Default|GetBPC_MultiToolA)) false false))
        (:NewEnumerator1
          (Transformation|SetWorldLocation (Variables|Default|GetForwardAxe) (Transformation|GetWorldLocation (Variables|Default|GetBPC_MultiToolB)) false false))))))

(fn ConstructionScript)

(fn UpdateSubBatteryFillAmount
  (params (NewZSizeValue :type Float%20%28double-precision%29))
  (switch Utilities|FlowControl|Switch|SwitchonE_MultiToolType (Variables|Components|GetActiveMultiTool)
    (:NewEnumerator0
      (Transformation|SetRelativeScale3D (Variables|Default|GetFBX_SubBattery_FillPart_MultiToolA) (Math|Vector|MakeVector 1.0 1.0 NewZSizeValue)))
    (:NewEnumerator1
      (Transformation|SetRelativeScale3D (Variables|Default|GetFBX_SubBattery_FillPart_MultiToolB) (Math|Vector|MakeVector 1.0 1.0 NewZSizeValue)))))