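; BP_CH_MainMenu provides the main menu camera and turns it toward a given location.
; RotateCameraTo plays a timeline that lerps the camera along the shortest path to a look-at rotation, at fixed play rate, ignoring its TransitionDuration input.
; When the turn finishes, it finds the WBP_MainMenu widget and updates its confirm-button display to match the selected tutorial level option or none.
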(event Custom|RotateCameraTo
  (params (TargetLocation :type Vector) (TransitionDuration :type Float%20%28double-precision%29))
  (Variables|Default|SetCameraStartRotation (Transformation|GetWorldRotation (Variables|Default|GetCamera)))
  (Variables|Default|SetCameraTargetRotation (Math|Rotator|FindLookatRotation (Transformation|GetWorldLocation (Variables|Default|GetCamera)) TargetLocation))
  (Components|Timeline|SetPlayRate (Variables|Default|GetCameraRotation) 1.0)
  (bind _alpha (Timeline|CameraRotation PlayFromStart)
    (:Update
      (Transformation|SetWorldRotation (Variables|Default|GetCamera) (Math|Rotator|Lerp(Rotator) (Variables|Default|GetCameraStartRotation) (Variables|Default|GetCameraTargetRotation) _alpha true) false false))
    (:Finished
      (bind _foundwidgets (Widget|GetAllWidgetsOfClass "/Game/Script/UI/WBP_MainMenu.WBP_MainMenu_C" false))
      (switch Utilities|FlowControl|Switch|SwitchonE_MainMenuOptions (Variables|/Game/Script/UI/WBP_MainMenu.WBP_MainMenu_C|GetMainMenuOptions (Utilities|Array|Get(acopy) _foundwidgets))
        (:NewEnumerator0
          (Default|HandleConfirmButtonsDysplay (Utilities|Array|Get(acopy) _foundwidgets) "NewEnumerator0"))
        (:NewEnumerator1
          (Default|HandleConfirmButtonsDysplay (Utilities|Array|Get(acopy) _foundwidgets) "NewEnumerator1"))
        (:NewEnumerator2
          (Default|HandleConfirmButtonsDysplay (Utilities|Array|Get(acopy) _foundwidgets) "NewEnumerator2"))))))

(event EventBeginPlay)

(event Collision|EventActorBeginOverlap
  (params (OtherActor :type Actor%20Object%20Reference)))

(event EventTick
  (params (DeltaSeconds :type Float%20%28single-precision%29)))

(fn ConstructionScript)