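; Multi-tool weapon component that attaches to the first-person character's grip and provides hook shot, rope and discharge abilities.
; Shoot fires a cooldown-gated hook projectile.
; StickySplash cycles through two rope projectiles joined by a runtime cable, then clears them; once both anchor, a box collision actor spans the rope.
; Holding discharge sphere-traces each tick for another multi-tool, spawning or resetting the QTE discharge manager when both are linked.
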(event Custom|OnRopeAttached
  (params (Hit%20Scene%20Component :type Scene%20Component%20Object%20Reference) (Hit%20Location :type Vector))
  (bind _cable (Variables|Default|GetCable))
  (bind _numberofropeanchored (Variables|Default|GetNumberOfRopeAnchored))
  (bind _returnvalue (Transformation|GetWorldLocation _cable))
  (bind _returnvalue_2 (Class|CableComponent|GetAttachedComponent _cable))
  (bind _endlocation (Variables|/Script/CableComponent.CableComponent|GetEndLocation _cable))
  (bind _returnvalue_3 (Transformation|GetWorldLocation _returnvalue_2))
  (bind _returnvalue_4 (+ _returnvalue_3 _endlocation))
  (bind _returnvalue_5 (- _returnvalue_4 _returnvalue))
  (bind _returnvalue_6 (Math|Vector|Normalize _returnvalue_5))
  (bind _returnvalue_7 (/ _returnvalue_5 2.0))
  (bind _returnvalue_8 (Math|Conversions|RotationFromXVector _returnvalue_6))
  (bind _returnvalue_9 (Math|Vector|VectorLength _returnvalue_7))
  (Math|Integer|IncrementInt _numberofropeanchored
    (:%20%20
      (switch int _numberofropeanchored
        (:2
          (Collision|BoxTraceByChannel (Transformation|GetWorldLocation (Variables|Default|GetCable)) _returnvalue_4 (/ (Math|Vector|MakeVector _returnvalue_9 (Variables|Default|GetRope%20Collision%20Box%20Extent%20) 1e+01) 2.0) _returnvalue_8 "TraceTypeQuery1" false 0 "Persistent" true "(R=0.000000,G=0.236701,B=1.000000,A=1.000000)")
          (bind _returnvalue_10 (Game|SpawnActorfromClass "/Game/Script/MultiTools/MultiToolB/BP_RopeBoxCollision.BP_RopeBoxCollision_C" (Math|Transform|MakeTransform (+ _returnvalue_7 _returnvalue) _returnvalue_8 "1.000000,1.000000,1.000000") "Undefined" "MultiplyWithRoot" 0 0))
          (bind _output_get (Variables|Default|SetRopeCollisionBP _returnvalue_10))
          (Default|ChangeBoxSize _output_get _returnvalue_9 (Variables|Default|GetRope%20Collision%20Box%20Extent%20) 1e+01)
          (Development|PrintString "Hello"))))))

(event Input|EnhancedActionEvents|EnhancedInputActionIA_Shoot
  (params (ActionValue :type Boolean) (ElapsedSeconds :type Float%20%28double-precision%29) (TriggeredSeconds :type Float%20%28double-precision%29) (InputAction :type Input%20Action%20Object%20Reference :default "/Game/FirstPerson/Input/Actions/IA_Shoot.IA_Shoot"))
  (Utilities|FlowControl|DoOnce false :!label _label
    (:Completed
      (Game|SpawnActorfromClass "/Game/Script/MultiTools/MultiToolB/BP_HookProjectile.BP_HookProjectile_C" (Math|Transform|MakeTransform (+ (Transformation|GetSocketLocation "Ammo") "0.000000,0.000000,-20.000000") (Camera|GetCameraRotation (Game|GetPlayerCameraManager 0))) "Undefined" "MultiplyWithRoot" 0 (Variables|Default|GetHook%20Max%20Distance) (Components|GetOwner) (Variables|Default|GetHook%20Intensity) 0)
      (Utilities|FlowControl|Delay (Variables|Default|GetHookCooldown))
      (goto _label Reset))))

(event Input|EnhancedActionEvents|EnhancedInputActionIA_StickySplash
  (params (ActionValue :type Boolean) (ElapsedSeconds :type Float%20%28double-precision%29) (TriggeredSeconds :type Float%20%28double-precision%29) (InputAction :type Input%20Action%20Object%20Reference :default "/Game/FirstPerson/Input/Actions/IA_StickySplash.IA_StickySplash"))
  (bind _cable (Variables|Default|GetCable))
  (bind _ropecollisionbp (Variables|Default|GetRopeCollisionBP))
  (switch int (Variables|Default|GetRopeStateIndex)
    (:Default
      (Variables|Default|SetRopeStateIndex 0))
    (:0
      (bind _returnvalue (Game|SpawnActorfromClass "/Game/Script/MultiTools/MultiToolB/BP_RopeProjectile.BP_RopeProjectile_C" (Math|Transform|MakeTransform (+ (Transformation|GetSocketLocation "Ammo") "0.000000,0.000000,-20.000000") (Camera|GetCameraRotation (Game|GetPlayerCameraManager 0))) "Undefined" "MultiplyWithRoot" 0 self 0))
      (Utilities|Array|Add (Variables|Default|GetRopeAnchorBPTable) _returnvalue)
      (Math|Integer|IncrementInt (Variables|Default|GetRopeStateIndex)
        (:%20%20
          (Components|Activation|Activate _cable false)
          (Rendering|ToggleVisibility _cable false)
          (Transformation|AttachComponentToComponent (Variables|Default|GetCable) (Variables|/Game/Script/MultiTools/MultiToolB/BP_RopeProjectile.BP_RopeProjectile_C|GetRopeAnchor _returnvalue) "None" "KeepWorld" "KeepWorld" "KeepWorld" true)
          (Class|CableComponent|SetAttachEndto (Variables|Default|GetCable) (Variables|Default|GetOwnerObject) "None" "None"))))
    (:1
      (bind _returnvalue_2 (Game|SpawnActorfromClass "/Game/Script/MultiTools/MultiToolB/BP_RopeProjectile.BP_RopeProjectile_C" (Math|Transform|MakeTransform (+ (Transformation|GetSocketLocation "Ammo") "0.000000,0.000000,-20.000000") (Camera|GetCameraRotation (Game|GetPlayerCameraManager 0))) "Undefined" "MultiplyWithRoot" 0 self 0))
      (Utilities|Array|Add (Variables|Default|GetRopeAnchorBPTable) _returnvalue_2)
      (Math|Integer|IncrementInt (Variables|Default|GetRopeStateIndex)
        (:%20%20
          (Class|CableComponent|SetAttachEndto (Variables|Default|GetCable) _returnvalue_2 "RopeAnchor" "None"))))
    (:2
      (for _array_element (Variables|Default|GetRopeAnchorBPTable)
        (Utilities|IsValid _array_element
          (:Is%20Valid
            (Actor|DestroyActor _array_element))))
      (Variables|Default|SetRopeStateIndex 0)
      (Transformation|DetachFromComponent (Variables|Default|GetCable) "KeepWorld" "KeepWorld" "KeepWorld" true)
      (Transformation|SetWorldLocation (Variables|Default|GetCable) (Transformation|GetSocketLocation (Variables|/Script/Engine.Actor|GetRootComponent (Variables|Default|GetOwnerObject)) "Ammo") false false)
      (Rendering|ToggleVisibility (Variables|Default|GetCable) false)
      (Variables|Default|SetNumberOfRopeAnchored 0)
      (Utilities|Array|Clear (Variables|Default|GetRopeAnchorBPTable))
      (Utilities|IsValid _ropecollisionbp
        (:Is%20Valid
          (Actor|DestroyActor _ropecollisionbp))))))

(event Input|EnhancedActionEvents|EnhancedInputActionIA_EnterDischargeState
  (params (ActionValue :type Boolean) (ElapsedSeconds :type Float%20%28double-precision%29) (TriggeredSeconds :type Float%20%28double-precision%29) (InputAction :type Input%20Action%20Object%20Reference :default "/Game/FirstPerson/Input/Actions/IA_EnterDischargeState.IA_EnterDischargeState"))
  (bind _returnvalue (Game|GetPlayerController 0))
  ;[1 0 1 0.5] Enable/Disable Searching A Multi Tool State From E_DischargeState
  (:Started
    (|SetBy-RefVar (Variables|Default|GetDischargeState) "NewEnumerator1")
    (Input|SetIgnoreMoveInput _returnvalue true))
  (:Canceled
    (if (Utilities|Enum|Equal(Enum) (Variables|Default|GetDischargeState) "NewEnumerator1") :!label _label
      (Input|SetIgnoreMoveInput _returnvalue false)
      (Input|SetIgnoreLookInput _returnvalue false)
      (|SetBy-RefVar (Variables|Default|GetDischargeState) "NewEnumerator0")))
  (:Completed
    (goto _label)))

(event EventBeginPlay
  (Utilities|FlowControl|Sequence
    (:then_0
      (bind _output_get (Variables|Default|SetOwnerObject (Components|GetOwner)))
      (bind _asbp_first_person_character (Utilities|Casting|CastToBP_FirstPersonCharacter _output_get))
      (Variables|Default|SetAs%20BP%20First%20Person%20Character _asbp_first_person_character)
      (Transformation|AttachComponentToComponent (Variables|/Game/FirstPerson/Blueprints/BP_FirstPersonCharacter.BP_FirstPersonCharacter_C|GetFirstPersonMesh _asbp_first_person_character) "GripPoint" "SnapToTarget" "SnapToTarget" "SnapToTarget" true)
      (bind _asplayer_controller (Utilities|Casting|CastToPlayerController (Pawn|GetController (Variables|Default|GetAs%20BP%20First%20Person%20Character))))
      (Utilities|IsValid (PlayerController|LocalPlayerSubsystems|GetEnhancedInputLocalPlayerSubsystem _asplayer_controller)
        (:Is%20Valid
          (Input|AddMappingContext (PlayerController|LocalPlayerSubsystems|GetEnhancedInputLocalPlayerSubsystem _asplayer_controller) "/Game/FirstPerson/Input/IMC_Weapons.IMC_Weapons" 0 "(bIgnoreAllPressedKeysUntilRelease=True,bForceImmediately=False,bNotifyUserSettings=False)")
          (bind _asfirst_person_anim_bp (Utilities|Casting|CastToFirstPerson_AnimBP (Components|SkeletalMesh|GetAnimInstance (Variables|/Game/FirstPerson/Blueprints/BP_FirstPersonCharacter.BP_FirstPersonCharacter_C|GetFirstPersonMesh (Variables|Default|GetAs%20BP%20First%20Person%20Character)))))
          (Variables|/Game/FirstPersonArms/Animations/FirstPerson_AnimBP.FirstPerson_AnimBP_C|SetHasRifle _asfirst_person_anim_bp true))))
    (:then_1
      (bind _returnvalue (Game|AddComponentbyClass (Variables|Default|GetOwnerObject) "/Script/CableComponent.CableComponent" false))
      (Variables|Default|SetCable _returnvalue)
      (Transformation|AttachComponentToComponent (Variables|Default|GetCable) (Variables|/Script/Engine.Actor|GetRootComponent (Variables|Default|GetOwnerObject)) "None" "KeepRelative" "KeepRelative" "KeepRelative" true))
    (:then_2
      (EventDispatchers|BindEventtoOnRopeAttachedDispatcher (delegate Custom|OnRopeAttached)))
    (:then_3
      (Components|Activation|Deactivate (Variables|Default|GetCable))
      (Rendering|ToggleVisibility (Variables|Default|GetCable) false))))

(event EventTick
  (params (DeltaSeconds :type Float%20%28single-precision%29))
  (bind _self self)
  (bind _returnvalue (Components|GetOwner _self))
  (Utilities|FlowControl|Sequence
    (:then_0
      ;[0.15 0.15 0.15 0.5] Doesn't work
      (if (> (Variables|Default|GetRopeStateIndex) 0)
        (Variables|/Script/CableComponent.CableComponent|SetCableLength (Variables|Default|GetCable) (Math|Vector|VectorLength (- (Transformation|GetWorldLocation (Class|CableComponent|GetAttachedComponent (Variables|Default|GetCable))) (+ (Variables|/Script/CableComponent.CableComponent|GetEndLocation (Variables|Default|GetCable)) (Transformation|GetActorLocation (Class|CableComponent|GetAttachedActor (Variables|Default|GetCable)))))))))
    (:then_1
      ;[1 1 0 0.5] Cast A Beam In Front Of The Player While In SearchingForAMultiToolState
      (if (Utilities|Enum|Equal(Enum) (Variables|Default|GetDischargeState) "NewEnumerator1")
        (bind _asbp_first_person_character (Utilities|Casting|CastToBP_FirstPersonCharacter _returnvalue)
          (:then
            (bind (_outhit _returnvalue_2) (Collision|SphereTraceByChannel (Transformation|GetWorldLocation (Variables|/Game/FirstPerson/Blueprints/BP_FirstPersonCharacter.BP_FirstPersonCharacter_C|GetFirstPersonCamera _asbp_first_person_character)) (+ (Transformation|GetWorldLocation (Variables|/Game/FirstPerson/Blueprints/BP_FirstPersonCharacter.BP_FirstPersonCharacter_C|GetFirstPersonCamera _asbp_first_person_character)) (* (Math|Vector|GetForwardVector (Variables|/Game/FirstPerson/Blueprints/BP_FirstPersonCharacter.BP_FirstPersonCharacter_C|GetFirstPersonCamera _asbp_first_person_character)) (* (Variables|Default|GetQTEStateDischargeActivationRange%28m%29) 100))) 3e+01 "TraceTypeQuery1" false 0 "ForDuration"))
            (if _returnvalue_2
              ;[0.003 1 0 0.5] Spawn BP_QTEDischargeManager If The MultiTools Are Linked
              (bind _asbpc_multi_tool_a (Utilities|Casting|CastToBPC_MultiToolA (Transformation|GetAttachParent (.HitComponent (Collision|BreakHitResult _outhit))))
                (:then
                  (Variables|Components|SetIsHittingAnotherMultitool true)
                  (if (Variables|/Game/Script/MultiTools/MultiToolA/BPC_MultiToolA.BPC_MultiToolA_C|GetIsHittingAnotherMultitool _asbpc_multi_tool_a)
                    (Variables|Default|SetDischargeState "NewEnumerator2" :!label _label)
                    (bind _returnvalue_3 (Actor|GetActorOfClass "/Game/Script/Discharge/BP_QTEDischargeManager.BP_QTEDischargeManager_C"))
                    (Utilities|IsValid _returnvalue_3
                      (:Is%20Valid
                        (if (not (Variables|/Game/Script/Discharge/WBP_QTEDischargeManager.WBP_QTEDischargeManager_C|GethasAlreadyBeenReset (Variables|/Game/Script/Discharge/BP_QTEDischargeManager.BP_QTEDischargeManager_C|GetQTEDischargeWidget _returnvalue_3)))
                          (Default|ResettheWidget (Variables|/Game/Script/Discharge/BP_QTEDischargeManager.BP_QTEDischargeManager_C|GetQTEDischargeWidget _returnvalue_3))))
                      (:Is%20Not%20Valid
                        (Game|SpawnActorfromClass "/Game/Script/Discharge/BP_QTEDischargeManager.BP_QTEDischargeManager_C" (Math|Transform|MakeTransform "0, 0, 0" "0, 0, 0" "1.000000,1.000000,1.000000") "Undefined" "MultiplyWithRoot" 0 0)))))
                (:CastFailed
                  (bind _asbpc_multi_tool_b (Utilities|Casting|CastToBPC_MultiToolB (Transformation|GetAttachParent (.HitComponent (Collision|BreakHitResult _outhit)))))
                  (Variables|Components|SetIsHittingAnotherMultitool true)
                  (if (Variables|BPC_MultiToolB_C|GetIsHittingAnotherMultitool _asbpc_multi_tool_b)
                    (goto _label))))))
          (:CastFailed
            (bind _asbp_multi_tool_waiting_for_discharge_qte (Utilities|Casting|CastToBP_MultiToolWaitingForDischargeQTE _returnvalue))
            (bind (_outhit_2 _returnvalue_4) (Collision|SphereTraceByChannel (Transformation|GetWorldLocation (Variables|/Game/Script/MultiTools/BP_MultiToolWaitingForDischargeQTE.BP_MultiToolWaitingForDischargeQTE_C|GetForwardAxe _asbp_multi_tool_waiting_for_discharge_qte)) (+ (Transformation|GetWorldLocation (Variables|/Game/Script/MultiTools/BP_MultiToolWaitingForDischargeQTE.BP_MultiToolWaitingForDischargeQTE_C|GetForwardAxe _asbp_multi_tool_waiting_for_discharge_qte)) (* (Math|Vector|GetForwardVector (Variables|/Game/Script/MultiTools/BP_MultiToolWaitingForDischargeQTE.BP_MultiToolWaitingForDischargeQTE_C|GetForwardAxe _asbp_multi_tool_waiting_for_discharge_qte)) (* (Variables|Default|GetQTEStateDischargeActivationRange%28m%29) 100))) 3e+01 "TraceTypeQuery1" false 0 "ForDuration"))
            (if _returnvalue_4
              (bind _asbpc_multi_tool_a_2 (Utilities|Casting|CastToBPC_MultiToolA (Transformation|GetAttachParent (.HitComponent (Collision|BreakHitResult _outhit_2))))
                (:then
                  (Variables|Components|SetIsHittingAnotherMultitool true)
                  (if (Variables|/Game/Script/MultiTools/MultiToolA/BPC_MultiToolA.BPC_MultiToolA_C|GetIsHittingAnotherMultitool _asbpc_multi_tool_a_2)
                    (goto _label)))
                (:CastFailed
                  (bind _asbpc_multi_tool_b_2 (Utilities|Casting|CastToBPC_MultiToolB (Transformation|GetAttachParent (.HitComponent (Collision|BreakHitResult _outhit_2)))))
                  (Variables|Components|SetIsHittingAnotherMultitool true)
                  (if (Variables|BPC_MultiToolB_C|GetIsHittingAnotherMultitool _asbpc_multi_tool_b_2)
                    (goto _label)))))))))))