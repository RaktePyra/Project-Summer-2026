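; Hook projectile that flies out on a cable tethered to its owner, then homes back and destroys itself on overlapping the owner.
; Tick sizes the cable to travel distance and starts the return at max range, re-aiming velocity at the owner every frame.
; Outbound box overlaps either message BPI_Hookable actors and start the return, or tug other movable primitives toward the owner with an upward-biased impulse, without triggering return.
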(event OnComponentBeginOverlap(Box)
  (params (OverlappedComponent :type Primitive%20Component%20Object%20Reference) (OtherActor :type Actor%20Object%20Reference) (OtherComp :type Primitive%20Component%20Object%20Reference) (OtherBodyIndex :type Integer) (bFromSweep :type Boolean) (SweepResult :type Hit%20Result%20Structure%20%28by%20ref%29))
  (bind _projectilemovement (Variables|Default|GetProjectileMovement))
  (if (not (Variables|Default|GetisReturning))
    (if (not (or (== (Variables|Default|GetOwnerActor) OtherActor) (== OtherActor self)))
      (Variables|Default|SetHit%20Actor OtherActor)
      (if (Utilities|DoesObjectImplementInterface (Variables|Default|GetHit%20Actor) "/Game/Script/MultiTools/MultiToolB/BPI_Hookable.BPI_Hookable_C")
        (Class|BPIHookable|Hook(Message) (Variables|Default|GetHit%20Actor))
        (Variables|/Script/Engine.MovementComponent|SetVelocity _projectilemovement (* (Variables|/Script/Engine.MovementComponent|GetVelocity _projectilemovement) -1.0))
        (Variables|Default|SetisReturning true)
        (else
          (switch Utilities|FlowControl|Switch|SwitchonEComponentMobility (Variables|/Script/Engine.SceneComponent|GetMobility (Variables|/Script/Engine.Actor|GetRootComponent (Variables|Default|GetHit%20Actor)))
            (:Movable
              (bind _asprimitive_component (Utilities|Casting|CastToPrimitiveComponent (Variables|/Script/Engine.Actor|GetRootComponent (Variables|Default|GetHit%20Actor))))
              (Physics|AddImpulse _asprimitive_component (* (Math|Vector|MakeVector (.X (Math|Vector|BreakVector (Math|Vector|Normalize (- (Transformation|GetActorLocation (Variables|Default|GetOwnerActor)) (Transformation|GetActorLocation (Variables|Default|GetHit%20Actor)))))) (.Y (Math|Vector|BreakVector (Math|Vector|Normalize (- (Transformation|GetActorLocation (Variables|Default|GetOwnerActor)) (Transformation|GetActorLocation (Variables|Default|GetHit%20Actor)))))) 1.0) (* (Variables|Default|GetHook%20Intensity) (Variables|Default|GetHookScalingFactor%20))) "None" false))))))
    (elif (== OtherActor (Variables|Default|GetOwnerActor))
      (Actor|DestroyActor))))

(event EventBeginPlay
  (Variables|Default|SetHookHeadStartPosition (Transformation|GetWorldLocation (Variables|Default|GetHookHead)))
  (Variables|Default|SetHookDirection (Math|Vector|Normalize (Math|Vector|RotateVector "1.000000,0.000000,0.000000" (Camera|GetCameraRotation (Game|GetPlayerCameraManager 0)))))
  (Class|CableComponent|SetAttachEndtoComponent (Variables|Default|GetCable) (Variables|Default|GetHookHead) "None")
  (Transformation|AttachComponentToComponent (Variables|Default|GetCable) (Variables|/Script/Engine.Actor|GetRootComponent (Variables|Default|GetOwnerActor)) "None" "KeepWorld" "KeepWorld" "KeepWorld" false))

(event Collision|EventActorBeginOverlap
  (params (OtherActor :type Actor%20Object%20Reference)))

(event EventTick
  (params (DeltaSeconds :type Float%20%28single-precision%29))
  (bind _projectilemovement (Variables|Default|GetProjectileMovement))
  (bind _hookhead (Variables|Default|GetHookHead))
  (bind _hookheadstartposition (Variables|Default|GetHookHeadStartPosition))
  (bind _returnvalue (Transformation|GetWorldLocation _hookhead))
  (bind _returnvalue_2 (- _returnvalue _hookheadstartposition))
  (bind _returnvalue_3 (Math|Vector|VectorLength _returnvalue_2))
  (if (not (Variables|Default|GetisReturning))
    _
    (else
      (Variables|/Script/Engine.MovementComponent|SetVelocity (Variables|Default|GetProjectileMovement) (* (Math|Vector|Normalize (- (Transformation|GetActorLocation (Variables|Default|GetOwnerActor)) (Transformation|GetActorLocation))) (Math|Vector|VectorLength (Variables|/Script/Engine.MovementComponent|GetVelocity (Variables|Default|GetProjectileMovement)))))))
  (Variables|/Script/CableComponent.CableComponent|SetCableLength (Variables|Default|GetCable) (Math|Float|Min(Float) (Variables|Default|GetHookMaxDistance) _returnvalue_3))
  (if (> _returnvalue_3 (Variables|Default|GetHookMaxDistance))
    (Utilities|FlowControl|DoOnce false
      (:Completed
        (Variables|/Script/Engine.MovementComponent|SetVelocity _projectilemovement (* (Variables|/Script/Engine.MovementComponent|GetVelocity _projectilemovement) -1.0))
        (Variables|Default|SetisReturning true)))))

(fn ConstructionScript)