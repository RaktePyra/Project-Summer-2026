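; Rope projectile for MultiTool B that reports an attachment to its owning multitool on overlap.
; When its box overlaps anything but the tool's owner, it line-traces from the cone toward its forward vector times 100, without adding the start location.
; It passes the impact point and its own overlapped component to the rope-attached dispatcher, then zeroes its velocity and disables box overlaps.
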(event OnComponentBeginOverlap(Box)
  (params (OverlappedComponent :type Primitive%20Component%20Object%20Reference) (OtherActor :type Actor%20Object%20Reference) (OtherComp :type Primitive%20Component%20Object%20Reference) (OtherBodyIndex :type Integer) (bFromSweep :type Boolean) (SweepResult :type Hit%20Result%20Structure%20%28by%20ref%29))
  (if (!= OtherActor (Variables|/Game/Script/MultiTools/MultiToolB/BPC_MultiToolB.BPC_MultiToolB_C|GetOwnerObject (Variables|Default|GetOwnerMultiTool)))
    (bind _outhit (Collision|LineTraceByChannel (Transformation|GetWorldLocation (Variables|Default|GetCone)) (* (Math|Vector|GetForwardVector (Transformation|GetWorldRotation (Variables|Default|GetCone))) 1e+02) "TraceTypeQuery1" false 0 "ForDuration"))
    (Default|CallOnRopeAttachedDispatcher (Variables|Default|GetOwnerMultiTool) OverlappedComponent (.impactpoint _outhit))
    (Variables|/Script/Engine.MovementComponent|SetVelocity (Variables|Default|GetProjectileMovement) "0, 0, 0")
    (Variables|/Script/Engine.PrimitiveComponent|SetbGenerateOverlapEvents (Variables|Default|GetBox) false)))

(event EventTick
  (params (DeltaSeconds :type Float%20%28single-precision%29)))

(fn ConstructionScript)