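; First-person MultiTool A weapon component that repels objects, fires sticky splash projectiles and links with other multitools.
; Attaches to the character's grip socket, with tuning loaded from and saved to a SaveGame slot.
; Shooting uses a box-trace cone with distance falloff or a sphere-trace ray, calling IRepulsable or adding impulses.
; In discharge state, Tick sphere-traces for a multitool hitting back, then spawns or resets the QTE manager.
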(event Custom|Save%20Loadout
  (bind _returnvalue (SaveGame|CreateSaveGameObject "/Game/Script/BP_SaveGameObject.BP_SaveGameObject_C"))
  (Variables|/Game/Script/BP_SaveGameObject.BP_SaveGameObject_C|SetMultiToolALoadout _returnvalue (Utilities|Struct|MakeS_MultiToolConfig (Variables|ConfigA|GetBox%20Radius%20for%20Impulse%20Detection%20A) (Variables|ConfigA|GetImpulsion%20Intensity%20A) (Variables|ConfigA|GetCone%20Angle%20A) (Variables|ConfigA|GetCone%20Radius) (Variables|ConfigB|GetRayRadiusB) (Variables|ConfigB|GetRayLength) (Variables|ConfigB|GetImpulsion%20Intensity%20B)))
  (SaveGame|SaveGametoSlot _returnvalue "MultitoolA"))

(event Input|EnhancedActionEvents|EnhancedInputActionIA_Shoot
  (params (ActionValue :type Boolean) (ElapsedSeconds :type Float%20%28double-precision%29) (TriggeredSeconds :type Float%20%28double-precision%29) (InputAction :type Input%20Action%20Object%20Reference :default "/Game/FirstPerson/Input/Actions/IA_Shoot.IA_Shoot"))
  (bind _ownergameobject (Variables|Default|GetOwnerGameObject))
  (bind _ownergameobject_2 (Variables|Default|GetOwnerGameObject))
  (bind _box_radius_for_impulse_detection_a (Variables|ConfigA|GetBox%20Radius%20for%20Impulse%20Detection%20A))
  (bind _ownergameobject_3 (Variables|Default|GetOwnerGameObject))
  (bind _cone_angle_a (Variables|ConfigA|GetCone%20Angle%20A))
  (bind _returnvalue (Transformation|GetActorLocation _ownergameobject))
  (bind _returnvalue_2 (Actor|GetComponentbyClass _ownergameobject_2 "/Script/Engine.CameraComponent"))
  (bind _returnvalue_3 (Actor|GetComponentbyClass _ownergameobject_3 "/Script/Engine.CameraComponent"))
  (:Triggered
    (if (Variables|Default|GetIsConfigurationA)
      (Utilities|IsValid _returnvalue_3
        (:Is%20Valid
          (Variables|Default|SetRotationToUseForTrace (Transformation|GetWorldRotation _returnvalue_3)))
        (:Is%20Not%20Valid
          (Variables|Default|SetRotationToUseForTrace (Transformation|GetActorRotation (Variables|Default|GetOwnerGameObject)))))
      (bind _outhits (Class|KismetSystemLibrary|BoxTraceMulti (+ (Transformation|GetActorLocation (Variables|Default|GetOwnerGameObject)) (Math|Vector|RotateVector (Math|Vector|MakeVector (Variables|ConfigA|GetBox%20Radius%20for%20Impulse%20Detection%20A) 0.0 0.0) (Variables|Default|GetRotationToUseForTrace))) (+ (Transformation|GetActorLocation (Variables|Default|GetOwnerGameObject)) (Math|Vector|RotateVector (Math|Vector|MakeVector (Variables|ConfigA|GetBox%20Radius%20for%20Impulse%20Detection%20A) 0.0 0.0) (Variables|Default|GetRotationToUseForTrace))) (Math|Vector|MakeVector _box_radius_for_impulse_detection_a _box_radius_for_impulse_detection_a _box_radius_for_impulse_detection_a) (Variables|Default|GetRotationToUseForTrace) "TraceTypeQuery1" false 0 "ForDuration" true))
      (for _array_element _outhits
        (Variables|Default|SetHit%20Actor%20A (.HitActor (Collision|BreakHitResult _array_element)))
        (if (and (<= (Class|KismetMathLibrary|DegAcos (Math|Vector|DotProduct (* (Math|Vector|Normalize (- (Transformation|GetActorLocation (Variables|Default|GetHit%20Actor%20A)) (Transformation|GetActorLocation (Variables|Default|GetOwnerGameObject)))) (Variables|ConfigA|GetImpulsion%20Intensity%20A)) (Math|Rotator|GetRotationXVector (Variables|Default|GetRotationToUseForTrace)))) _cone_angle_a) (>= (Class|KismetMathLibrary|DegAcos (Math|Vector|DotProduct (* (Math|Vector|Normalize (- (Transformation|GetActorLocation (Variables|Default|GetHit%20Actor%20A)) (Transformation|GetActorLocation (Variables|Default|GetOwnerGameObject)))) (Variables|ConfigA|GetImpulsion%20Intensity%20A)) (Math|Rotator|GetRotationXVector (Variables|Default|GetRotationToUseForTrace)))) (* _cone_angle_a -1.0)))
          (if (<= (Math|Vector|VectorLength (- (.Location (Collision|BreakHitResult _array_element)) (Transformation|GetActorLocation (Variables|Default|GetOwnerGameObject)))) (Variables|ConfigA|GetCone%20Radius))
            (if (Utilities|DoesObjectImplementInterface (Variables|Default|GetHit%20Actor%20A) "/Game/Script/MultiTools/MultiToolA/IRepulsable.IRepulsable_C")
              (Class|IRepulsable|Repulse(Message) (Variables|Default|GetHit%20Actor%20A))
              (elif (Physics|IsSimulatingPhysics (Variables|/Script/Engine.Actor|GetRootComponent (Variables|Default|GetHit%20Actor%20A)) "None")
                (bind _asprimitive_component (Utilities|Casting|CastToPrimitiveComponent (Variables|/Script/Engine.Actor|GetRootComponent (Variables|Default|GetHit%20Actor%20A))))
                (Physics|AddImpulse _asprimitive_component (* (* (* (Math|Vector|Normalize (- (Transformation|GetActorLocation (Variables|Default|GetHit%20Actor%20A)) (Transformation|GetActorLocation (Variables|Default|GetOwnerGameObject)))) (Variables|ConfigA|GetImpulsion%20Intensity%20A)) 1e+05) (- 1.0 (Math|Float|Clamp(Float) (Math|Float|Square (/ (Math|Vector|VectorLength (- (Transformation|GetActorLocation (Variables|Default|GetHit%20Actor%20A)) (Transformation|GetActorLocation (Variables|Default|GetOwnerGameObject)))) (Variables|ConfigA|GetCone%20Radius)))))) "None" false)
                (Development|PrintString (Utilities|String|ToString(Float) (Math|Float|Clamp(Float) (Math|Float|Square (/ (Math|Vector|VectorLength (- (Transformation|GetActorLocation (Variables|Default|GetHit%20Actor%20A)) (Transformation|GetActorLocation (Variables|Default|GetOwnerGameObject)))) (Variables|ConfigA|GetCone%20Radius)))))))))))))
  (:Ongoing
    (if (not (Variables|Default|GetIsConfigurationA))
      (Utilities|IsValid _returnvalue_2
        (:Is%20Valid
          (Variables|Default|SetRotationToUseForTrace (Transformation|GetWorldRotation _returnvalue_2)))
        (:Is%20Not%20Valid
          (Variables|Default|SetRotationToUseForTrace (Transformation|GetActorRotation (Variables|Default|GetOwnerGameObject)))))
      (bind _outhit (Collision|SphereTraceByChannel _returnvalue (+ _returnvalue (* (Math|Vector|GetForwardVector _returnvalue_2) (Variables|ConfigB|GetRayLength))) (Variables|ConfigB|GetRayRadiusB) "TraceTypeQuery1" false 0 "ForDuration"))
      (bind _output_get (Variables|Default|SetHit%20Actor%20B (.hitactor _outhit)))
      (Utilities|IsValid _output_get
        (:Is%20Valid
          (if (Utilities|DoesObjectImplementInterface _output_get "/Game/Script/MultiTools/MultiToolA/IRepulsable.IRepulsable_C")
            (Class|IRepulsable|Repulse(Message) (Variables|Default|GetHit%20Actor%20B))
            (else
              (Utilities|IsValid (Variables|/Script/Engine.Actor|GetRootComponent (Variables|Default|GetHit%20Actor%20B))
                (:Is%20Valid
                  (bind _asprimitive_component_2 (Utilities|Casting|CastToPrimitiveComponent (Variables|/Script/Engine.Actor|GetRootComponent (Variables|Default|GetHit%20Actor%20B))))
                  (Physics|AddImpulse _asprimitive_component_2 (* (* (Math|Vector|Normalize (- (Transformation|GetActorLocation (Variables|Default|GetHit%20Actor%20B)) (Transformation|GetActorLocation (Variables|Default|GetOwnerGameObject)))) (Variables|ConfigB|GetImpulsion%20Intensity%20B)) 1e+05) "None" false))))))))))

(event Input|EnhancedActionEvents|EnhancedInputActionIA_StickySplash
  (params (ActionValue :type Boolean) (ElapsedSeconds :type Float%20%28double-precision%29) (TriggeredSeconds :type Float%20%28double-precision%29) (InputAction :type Input%20Action%20Object%20Reference :default "/Game/FirstPerson/Input/Actions/IA_StickySplash.IA_StickySplash"))
  (bind _returnvalue (Game|GetPlayerCameraManager 0))
  (bind _returnvalue_2 (Transformation|GetSocketLocation "Ammo"))
  (bind _projectile_offset (Variables|Default|GetProjectile%20Offset))
  (bind _returnvalue_3 (Camera|GetCameraRotation _returnvalue))
  (bind _returnvalue_4 (Math|Vector|RotateVector _projectile_offset _returnvalue_3))
  (bind _returnvalue_5 (+ _returnvalue_2 _returnvalue_4))
  (if (Utilities|IsValid (Variables|Default|GetActive%20Sticky%20Surface))
    (Actor|DestroyActor (Variables|Default|GetActive%20Sticky%20Surface))
    (Variables|Default|SetActive%20Sticky%20Surface 0)
    (else
      (bind _returnvalue_6 (Game|SpawnActorfromClass "/Game/Script/MultiTools/MultiToolA/BP_StickySplashProjectile.BP_StickySplashProjectile_C" (Math|Transform|MakeTransform _returnvalue_5 _returnvalue_3) "Undefined" "OverrideRootScale" 0 0))
      (Variables|/Game/Script/MultiTools/MultiToolA/BP_StickySplashProjectile.BP_StickySplashProjectile_C|SetGunOrigin _returnvalue_6 self)
      (Audio|PlaySoundatLocation "/Game/FPWeapon/Audio/FirstPersonTemplateWeaponFire02.FirstPersonTemplateWeaponFire02" _returnvalue_5 "0, 0, 0" 1.0 1.0 0.0 0 0 0 0) ; Play firing sound
    )))

(event Input|EnhancedActionEvents|EnhancedInputActionIA_EnterDischargeState
  (params (ActionValue :type Boolean) (ElapsedSeconds :type Float%20%28double-precision%29) (TriggeredSeconds :type Float%20%28double-precision%29) (InputAction :type Input%20Action%20Object%20Reference :default "/Game/FirstPerson/Input/Actions/IA_EnterDischargeState.IA_EnterDischargeState"))
  (bind _returnvalue (Game|GetPlayerController 0))
  ;[1 0 1 0.5] Enable/Disable Searching A Multi Tool State From E_DischargeState
  (:Started
    (if (Utilities|Enum|Equal(Enum) (Variables|Default|GetDischargeState) "NewEnumerator0")
      (|SetBy-RefVar (Variables|Default|GetDischargeState) "NewEnumerator1")
      (Input|SetIgnoreMoveInput _returnvalue true)))
  (:Canceled
    (if (Utilities|Enum|Equal(Enum) (Variables|Default|GetDischargeState) "NewEnumerator1") :!label _label
      (Input|SetIgnoreMoveInput _returnvalue false)
      (Input|SetIgnoreLookInput _returnvalue false)
      (|SetBy-RefVar (Variables|Default|GetDischargeState) "NewEnumerator0")))
  (:Completed
    (goto _label)))

(event EventBeginPlay
  (bind _returnvalue (Components|GetOwner))
  (bind _returnvalue_2 (SaveGame|LoadGamefromSlot "MultitoolA"))
  (Utilities|IsValid _returnvalue_2
    (:Is%20Valid
      (bind _asbp_save_game_object (Utilities|Casting|CastToBP_SaveGameObject _returnvalue_2)
        (:then
          (Variables|Default|SetMultiTool%20Loadout (Variables|/Game/Script/BP_SaveGameObject.BP_SaveGameObject_C|GetMultiToolALoadout _asbp_save_game_object))
          (Utilities|FlowControl|Sequence
            (:then_0
              (Variables|ConfigA|SetBox%20Radius%20for%20Impulse%20Detection%20A (.boxradiusforimpulsedetectiona (Variables|/Game/Script/BP_SaveGameObject.BP_SaveGameObject_C|GetMultiToolALoadout _asbp_save_game_object))))
            (:then_1
              (Variables|ConfigA|SetImpulsion%20Intensity%20A (.impulsionintensitya (Variables|/Game/Script/BP_SaveGameObject.BP_SaveGameObject_C|GetMultiToolALoadout _asbp_save_game_object))))
            (:then_2
              (Variables|ConfigA|SetCone%20Angle%20A (.coneanglea (Variables|/Game/Script/BP_SaveGameObject.BP_SaveGameObject_C|GetMultiToolALoadout _asbp_save_game_object))))
            (:then_3
              (Variables|ConfigA|SetCone%20Radius (.coneradius (Variables|/Game/Script/BP_SaveGameObject.BP_SaveGameObject_C|GetMultiToolALoadout _asbp_save_game_object))))
            (:then_4
              (Variables|ConfigB|SetRayRadiusB (.rayradiusb (Variables|/Game/Script/BP_SaveGameObject.BP_SaveGameObject_C|GetMultiToolALoadout _asbp_save_game_object))))
            (:then_5
              (Variables|ConfigB|SetRayLength (.raylength (Variables|/Game/Script/BP_SaveGameObject.BP_SaveGameObject_C|GetMultiToolALoadout _asbp_save_game_object))))
            (:then_6
              (Variables|ConfigB|SetImpulsion%20Intensity%20B (.impulsionintensityb (Variables|/Game/Script/BP_SaveGameObject.BP_SaveGameObject_C|GetMultiToolALoadout _asbp_save_game_object)))
              (Variables|Default|SetOwnerGameObject _returnvalue :!label _label)
              (bind _asbp_first_person_character (Utilities|Casting|CastToBP_FirstPersonCharacter _returnvalue))
              (Variables|Default|SetAs%20BP%20First%20Person%20Character _asbp_first_person_character)
              (Transformation|AttachComponentToComponent (Variables|/Game/FirstPerson/Blueprints/BP_FirstPersonCharacter.BP_FirstPersonCharacter_C|GetFirstPersonMesh _asbp_first_person_character) "GripPoint" "SnapToTarget" "SnapToTarget" "SnapToTarget" true)
              (bind _asplayer_controller (Utilities|Casting|CastToPlayerController (Pawn|GetController (Variables|Default|GetAs%20BP%20First%20Person%20Character))))
              (Utilities|IsValid (PlayerController|LocalPlayerSubsystems|GetEnhancedInputLocalPlayerSubsystem _asplayer_controller)
                (:Is%20Valid
                  (Input|AddMappingContext (PlayerController|LocalPlayerSubsystems|GetEnhancedInputLocalPlayerSubsystem _asplayer_controller) "/Game/FirstPerson/Input/IMC_Weapons.IMC_Weapons" 0 "(bIgnoreAllPressedKeysUntilRelease=True,bForceImmediately=False,bNotifyUserSettings=False)")
                  (bind _asfirst_person_anim_bp (Utilities|Casting|CastToFirstPerson_AnimBP (Components|SkeletalMesh|GetAnimInstance (Variables|/Game/FirstPerson/Blueprints/BP_FirstPersonCharacter.BP_FirstPersonCharacter_C|GetFirstPersonMesh (Variables|Default|GetAs%20BP%20First%20Person%20Character)))))
                  (Variables|/Game/FirstPersonArms/Animations/FirstPerson_AnimBP.FirstPerson_AnimBP_C|SetHasRifle _asfirst_person_anim_bp true))))))
        (:CastFailed
          (goto _label))))
    (:Is%20Not%20Valid
      (goto _label))))

(event EventTick
  (params (DeltaSeconds :type Float%20%28single-precision%29))
  (bind _self self)
  (bind _returnvalue (Components|GetOwner _self))
  ;[1 1 0 0.5] Cast A Beam In Front Of The Player While In SearchingForAMultiToolState
  (Variables|Default|SetIsHittingAnotherMultitool false)
  (if (Utilities|Enum|Equal(Enum) (Variables|Default|GetDischargeState) "NewEnumerator1")
    (bind _asbp_first_person_character (Utilities|Casting|CastToBP_FirstPersonCharacter _returnvalue)
      (:then
        (bind (_outhit _returnvalue_2) (Collision|SphereTraceByChannel (Transformation|GetWorldLocation (Variables|/Game/FirstPerson/Blueprints/BP_FirstPersonCharacter.BP_FirstPersonCharacter_C|GetFirstPersonCamera _asbp_first_person_character)) (+ (Transformation|GetWorldLocation (Variables|/Game/FirstPerson/Blueprints/BP_FirstPersonCharacter.BP_FirstPersonCharacter_C|GetFirstPersonCamera _asbp_first_person_character)) (* (Math|Vector|GetForwardVector (Variables|/Game/FirstPerson/Blueprints/BP_FirstPersonCharacter.BP_FirstPersonCharacter_C|GetFirstPersonCamera _asbp_first_person_character)) (* (Variables|Default|GetQTEStateDischargeActivationRange%28m%29) 100))) 3e+01 "TraceTypeQuery1" false 0 "ForDuration"))
        (if _returnvalue_2
          ;[0.003 1 0 0.5] Spawn BP_QTEDischargeManager If The MultiTools Are Linked
          (bind _asbpc_multi_tool_a (Utilities|Casting|CastToBPC_MultiToolA (Transformation|GetAttachParent (.HitComponent (Collision|BreakHitResult _outhit))))
            (:then
              (Variables|Default|SetIsHittingAnotherMultitool true)
              (if (Variables|BPC_MultiToolA_C|GetIsHittingAnotherMultitool _asbpc_multi_tool_a)
                (Variables|Default|SetDischargeState "NewEnumerator2" :!label _label)
                (bind _returnvalue_3 (Actor|GetActorOfClass "/Game/Script/Discharge/BP_QTEDischargeManagerSpawner.BP_QTEDischargeManagerSpawner_C"))
                (Utilities|IsValid _returnvalue_3
                  (:Is%20Valid
                    (if (not (Variables|/Game/Script/Discharge/WBP_QTEDischargeManager.WBP_QTEDischargeManager_C|GethasAlreadyBeenReset (Variables|/Game/Script/Discharge/BP_QTEDischargeManagerSpawner.BP_QTEDischargeManagerSpawner_C|GetQTEDischargeWidget _returnvalue_3)))
                      (Default|ResettheWidget (Variables|/Game/Script/Discharge/BP_QTEDischargeManagerSpawner.BP_QTEDischargeManagerSpawner_C|GetQTEDischargeWidget _returnvalue_3))))
                  (:Is%20Not%20Valid
                    (Game|SpawnActorfromClass "/Game/Script/Discharge/BP_QTEDischargeManagerSpawner.BP_QTEDischargeManagerSpawner_C" (Math|Transform|MakeTransform "0, 0, 0" "0, 0, 0" "1.000000,1.000000,1.000000") "Undefined" "MultiplyWithRoot" 0 0)))))
            (:CastFailed
              (bind _asbpc_multi_tool_b (Utilities|Casting|CastToBPC_MultiToolB (Transformation|GetAttachParent (.HitComponent (Collision|BreakHitResult _outhit)))))
              (Variables|Default|SetIsHittingAnotherMultitool true)
              (if (Variables|/Game/Script/MultiTools/MultiToolB/BPC_MultiToolB.BPC_MultiToolB_C|GetIsHittingAnotherMultitool _asbpc_multi_tool_b)
                (goto _label))))))
      (:CastFailed
        (bind _asbp_multi_tool_waiting_for_discharge_qte (Utilities|Casting|CastToBP_MultiToolWaitingForDischargeQTE _returnvalue))
        (bind (_outhit_2 _returnvalue_4) (Collision|SphereTraceByChannel (Transformation|GetWorldLocation (Variables|/Game/Script/MultiTools/BP_MultiToolWaitingForDischargeQTE.BP_MultiToolWaitingForDischargeQTE_C|GetForwardAxe _asbp_multi_tool_waiting_for_discharge_qte)) (+ (Transformation|GetWorldLocation (Variables|/Game/Script/MultiTools/BP_MultiToolWaitingForDischargeQTE.BP_MultiToolWaitingForDischargeQTE_C|GetForwardAxe _asbp_multi_tool_waiting_for_discharge_qte)) (* (Math|Vector|GetForwardVector (Variables|/Game/Script/MultiTools/BP_MultiToolWaitingForDischargeQTE.BP_MultiToolWaitingForDischargeQTE_C|GetForwardAxe _asbp_multi_tool_waiting_for_discharge_qte)) (* (Variables|Default|GetQTEStateDischargeActivationRange%28m%29) 100))) 3e+01 "TraceTypeQuery1" false 0 "ForDuration"))
        (if _returnvalue_4
          (bind _asbpc_multi_tool_a_2 (Utilities|Casting|CastToBPC_MultiToolA (Transformation|GetAttachParent (.HitComponent (Collision|BreakHitResult _outhit_2))))
            (:then
              (Variables|Default|SetIsHittingAnotherMultitool true)
              (if (Variables|BPC_MultiToolA_C|GetIsHittingAnotherMultitool _asbpc_multi_tool_a_2)
                (goto _label)))
            (:CastFailed
              (bind _asbpc_multi_tool_b_2 (Utilities|Casting|CastToBPC_MultiToolB (Transformation|GetAttachParent (.HitComponent (Collision|BreakHitResult _outhit_2)))))
              (Variables|Default|SetIsHittingAnotherMultitool true)
              (if (Variables|/Game/Script/MultiTools/MultiToolB/BPC_MultiToolB.BPC_MultiToolB_C|GetIsHittingAnotherMultitool _asbpc_multi_tool_b_2)
                (goto _label)))))))))

(fn SetActiveStickyPlatform
  (params (NewParam :type BP%20Sticky%20Surface%20Object%20Reference))
  (Variables|Default|SetActive%20Sticky%20Surface NewParam))

(fn GetActiveStickySurface
  (return (Variables|Default|GetActive%20Sticky%20Surface)))

(fn RefreshGunConfig
  (params (New%20Configuration :type S%20Multi%20Tool%20Config%20Structure))
  (Utilities|FlowControl|Sequence
    (:then_0
      (Variables|ConfigA|SetBox%20Radius%20for%20Impulse%20Detection%20A (.boxradiusforimpulsedetectiona New%20Configuration)))
    (:then_1
      (Variables|ConfigA|SetImpulsion%20Intensity%20A (.impulsionintensitya New%20Configuration)))
    (:then_2
      (Variables|ConfigA|SetCone%20Angle%20A (.coneanglea New%20Configuration)))
    (:then_3
      (Variables|ConfigA|SetCone%20Radius (.coneradius New%20Configuration)))
    (:then_4
      (Variables|ConfigB|SetRayRadiusB (.rayradiusb New%20Configuration)))
    (:then_5
      (Variables|ConfigB|SetRayLength (.raylength New%20Configuration)))
    (:then_6
      (Variables|ConfigB|SetImpulsion%20Intensity%20B (.impulsionintensityb New%20Configuration)))))

(fn SaveConfigtoSlot
  (params (Config :type S%20Multi%20Tool%20Config%20Structure) (SlotName :type String))
  (bind _returnvalue (SaveGame|CreateSaveGameObject "/Game/Script/BP_SaveGameObject.BP_SaveGameObject_C"))
  (Variables|/Game/Script/BP_SaveGameObject.BP_SaveGameObject_C|SetMultiToolALoadout _returnvalue Config)
  (SaveGame|SaveGametoSlot _returnvalue SlotName))