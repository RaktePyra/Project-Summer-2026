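; BP_StickySplashProjectile is a MultiToolA projectile that leaves a sticky surface on whatever it hits.
; On BeginPlay it applies its initial speed and gravity scale to ProjectileMovement.
; On hit it destroys GunOrigin's active sticky surface, then spawns a normal-aligned BP_StickySurface and registers it with the gun, keeping only one active.
; The surface attaches to the hit actor, which receives StickyMessage before the projectile destroys itself.
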(event EventBeginPlay
  (Variables|/Script/Engine.ProjectileMovementComponent|SetInitialSpeed (Variables|Default|GetProjectileMovement) (Variables|Default|GetInitial%20Speed))
  (Variables|/Script/Engine.ProjectileMovementComponent|SetProjectileGravityScale (Variables|Default|GetProjectileMovement) (Variables|Default|GetProjectile%20Gravity%20Scale)))

(event Collision|EventActorBeginOverlap
  (params (OtherActor :type Actor%20Object%20Reference)))

(event EventTick
  (params (DeltaSeconds :type Float%20%28single-precision%29)))

(event Collision|EventHit
  (params (MyComp :type Primitive%20Component%20Object%20Reference) (Other :type Actor%20Object%20Reference) (OtherComp :type Primitive%20Component%20Object%20Reference) (bSelfMoved :type Boolean) (HitLocation :type Vector :default "0, 0, 0") (HitNormal :type Vector :default "0, 0, 0") (NormalImpulse :type Vector :default "0, 0, 0") (Hit :type Hit%20Result%20Structure%20%28by%20ref%29))
  (bind _active_sticky_surface (Default|GetActiveStickySurface (Variables|Default|GetGunOrigin)))
  (if (Utilities|IsValid _active_sticky_surface)
    (Actor|DestroyActor _active_sticky_surface))
  (bind _returnvalue (Game|SpawnActorfromClass "/Game/Script/MultiTools/MultiToolA/BP_StickySurface.BP_StickySurface_C" (Math|Transform|MakeTransform (+ HitLocation (* HitNormal 1.0)) (Math|Conversions|RotationFromXVector (.normal Hit))) "Undefined" "MultiplyWithRoot" 0 (.hitactor Hit) 0))
  (bind _output_get (Variables|/Game/Script/MultiTools/MultiToolA/BPC_MultiToolA.BPC_MultiToolA_C|SetActive%20Sticky%20Surface (Variables|Default|GetGunOrigin) _returnvalue))
  (Transformation|AttachActorToActor _output_get (.hitactor Hit) "None" "KeepWorld" "KeepWorld" "KeepWorld" true)
  (Class|IStickable|Sticky(Message) (.hitactor Hit))
  (Actor|DestroyActor))

(fn ConstructionScript)