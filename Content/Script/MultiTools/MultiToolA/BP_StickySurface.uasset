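; Sticky surface actor from MultiToolA that holds physics objects and characters in place while they overlap its box.
; Begin overlap disables gravity and physics simulation, zeroes character movement velocity and gravity, and removes the first-person player's default input mapping, tracking affected actors in an array.
; End overlap or destruction runs DisableStickynessOnActor to restore these states and send UnStickyMessage.
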(event OnComponentBeginOverlap(Box)
  (params (OverlappedComponent :type Primitive%20Component%20Object%20Reference) (OtherActor :type Actor%20Object%20Reference) (OtherComp :type Primitive%20Component%20Object%20Reference) (OtherBodyIndex :type Integer) (bFromSweep :type Boolean) (SweepResult :type Hit%20Result%20Structure%20%28by%20ref%29))
  (Variables|Default|SetOverlappingActor OtherActor)
  (Utilities|FlowControl|Sequence
    (:then_0
      (bind _asprimitive_component (Utilities|Casting|CastToPrimitiveComponent (Variables|/Script/Engine.Actor|GetRootComponent (Variables|Default|GetOverlappingActor))))
      (Physics|SetEnableGravity _asprimitive_component false)
      (if (Physics|IsSimulatingPhysics _asprimitive_component "None")
        (Physics|SetSimulatePhysics _asprimitive_component false)
        (Utilities|Array|AddUnique (Variables|Default|GetStickiedActorArray) (Variables|Default|GetOverlappingActor) :!label _label)))
    (:then_1
      (Utilities|IsValid (Actor|GetComponentbyClass (Variables|Default|GetOverlappingActor) "/Script/Engine.CharacterMovementComponent")
        (:Is%20Valid
          (Pawn|Components|CharacterMovement|ClearAccumulatedForces (Actor|GetComponentbyClass (Variables|Default|GetOverlappingActor) "/Script/Engine.CharacterMovementComponent"))
          (Variables|/Script/Engine.CharacterMovementComponent|SetGravityScale (Actor|GetComponentbyClass (Variables|Default|GetOverlappingActor) "/Script/Engine.CharacterMovementComponent") 0.0)
          (Variables|/Script/Engine.MovementComponent|SetVelocity (Actor|GetComponentbyClass (Variables|Default|GetOverlappingActor) "/Script/Engine.CharacterMovementComponent") "0, 0, 0")
          (goto _label))))
    (:then_2
      (bind _asbp_first_person_character (Utilities|Casting|CastToBP_FirstPersonCharacter (Variables|Default|GetOverlappingActor)))
      (Variables|Default|SetAs%20BP%20First%20Person%20Character _asbp_first_person_character)
      (bind _asplayer_controller (Utilities|Casting|CastToPlayerController (Pawn|GetController _asbp_first_person_character)))
      (bind _output_get (Variables|Default|SetAs%20Player%20Controller _asplayer_controller))
      (Utilities|IsValid (PlayerController|LocalPlayerSubsystems|GetEnhancedInputLocalPlayerSubsystem _output_get)
        (:Is%20Valid
          (Input|RemoveMappingContext (PlayerController|LocalPlayerSubsystems|GetEnhancedInputLocalPlayerSubsystem _output_get) "/Game/FirstPerson/Input/IMC_Default.IMC_Default" "(bIgnoreAllPressedKeysUntilRelease=True,bForceImmediately=False,bNotifyUserSettings=False)")
          (goto _label))))))

(event OnComponentEndOverlap(Box)
  (params (OverlappedComponent :type Primitive%20Component%20Object%20Reference) (OtherActor :type Actor%20Object%20Reference) (OtherComp :type Primitive%20Component%20Object%20Reference) (OtherBodyIndex :type Integer))
  (CallFunction|DisableStickynessonActor OtherActor))

(event EventBeginPlay)

(event EventDestroyed
  (bind _stickiedactorarray (Variables|Default|GetStickiedActorArray))
  (for _array_element _stickiedactorarray
    (CallFunction|DisableStickynessonActor _array_element))
  (Development|PrintString (Utilities|String|ToString(Integer) (Utilities|Array|Length _stickiedactorarray)))
  (Class|IStickable|UnSticky(Message) (Variables|Default|GetStickied%20Actor)))

(event EventTick
  (params (DeltaSeconds :type Float%20%28single-precision%29)))

(fn ConstructionScript)

(fn DisableStickynessonActor
  (params (Actor :type Actor%20Object%20Reference))
  (bind _returnvalue (Actor|GetComponentbyClass Actor "/Script/Engine.CharacterMovementComponent"))
  (Utilities|FlowControl|Sequence
    (:then_0
      (Utilities|IsValid _returnvalue
        (:Is%20Valid
          (Variables|/Script/Engine.CharacterMovementComponent|SetGravityScale _returnvalue 1.0)
          (Utilities|Array|RemoveItem (Variables|Default|GetStickiedActorArray) Actor :!label _label))))
    (:then_1
      (bind _asbp_first_person_character (Utilities|Casting|CastToBP_FirstPersonCharacter Actor)
        (:then
          (bind _asplayer_controller (Utilities|Casting|CastToPlayerController (Pawn|GetController _asbp_first_person_character)))
          (Utilities|IsValid (PlayerController|LocalPlayerSubsystems|GetEnhancedInputLocalPlayerSubsystem _asplayer_controller)
            (:Is%20Valid
              (Input|AddMappingContext (PlayerController|LocalPlayerSubsystems|GetEnhancedInputLocalPlayerSubsystem _asplayer_controller) "/Game/FirstPerson/Input/IMC_Default.IMC_Default" 0 "(bIgnoreAllPressedKeysUntilRelease=True,bForceImmediately=False,bNotifyUserSettings=False)")
              (goto _label))))
        (:CastFailed
          (bind _asprimitive_component (Utilities|Casting|CastToPrimitiveComponent (Variables|/Script/Engine.Actor|GetRootComponent Actor)))
          (Physics|SetEnableGravity _asprimitive_component true)
          (if (not (Physics|IsSimulatingPhysics _asprimitive_component "None"))
            (Physics|SetSimulatePhysics _asprimitive_component true)
            (goto _label)))))
    (:then_2
      (Class|IStickable|UnSticky(Message) Actor))))