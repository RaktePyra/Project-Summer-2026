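; Main battery actor that tracks cargo respawns as accumulated charge and triggers game over at the explosion limit.
; Tick spins the rotating mesh part faster with each respawn, using a per-respawn speed step computed on BeginPlay.
; Charge increases and resets update the sub-battery fill on the first-person character and, if present, the multitool waiting for discharge QTE.
; Reaching the limit shows the lose widget and switches input to UI only.
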(event EventBeginPlay
  ;[0 0 1 0.5] Set Battery Rotation Speed To Add
  (Variables|MainBatteryRotation|SetMainBatteryRotationSpeedToAdd (/ (- (Variables|MainBatteryRotation|GetMainBatteryMaxRotationSpeed) (Variables|MainBatteryRotation|GetMainBatteryRotationSpeed)) (Variables|Default|GetNumberOfRespawnBeforeExploding))))

(event EventTick
  (params (DeltaSeconds :type Float%20%28single-precision%29))
  ;[1 0 0 0.5] MainBatteryRotation
  (Transformation|AddWorldRotation (Variables|Default|GetFBX_MainBattery_RotatingPart) (Math|Rotator|MakeRotator 0.0 0.0 (+ (* (Variables|MainBatteryRotation|GetMainBatteryRotationSpeedToAdd) (Variables|Default|GetNumberOfTimeTheCargoHasRespawned)) (Variables|MainBatteryRotation|GetMainBatteryRotationSpeed))) false false))

(fn ConstructionScript)

(fn IncreaseBatteriesCharge
  (bind _numberoftimethecargohasrespawned (Variables|Default|GetNumberOfTimeTheCargoHasRespawned))
  (bind _numberofrespawnbeforeexploding (Variables|Default|GetNumberOfRespawnBeforeExploding))
  (bind _returnvalue (Math|Conversions|ToFloat(Integer) _numberofrespawnbeforeexploding))
  (bind _returnvalue_2 (Math|Conversions|ToFloat(Integer) _numberoftimethecargohasrespawned))
  (bind _returnvalue_3 (/ _returnvalue_2 _returnvalue))
  ;[0.992 0 0 0.5] Increase Batteries Charge
  (Math|Integer|IncrementInt (Variables|Default|GetNumberOfTimeTheCargoHasRespawned)
    (:%20%20
      ;[0 1 0 0.5] Update Sub Battery Fill Amount For BP_FirstPersonCharacter And BP_MultiToolWaitingForQTEDischarge
      (Utilities|FlowControl|Sequence
        (:then_0
          (bind _returnvalue_4 (Actor|GetActorOfClass "/Game/FirstPerson/Blueprints/BP_FirstPersonCharacter.BP_FirstPersonCharacter_C"))
          (Default|UpdateSubBatteryFillAmount _returnvalue_4 _returnvalue_3))
        (:then_1
          (bind _returnvalue_5 (Actor|GetActorOfClass "/Game/Script/MultiTools/BP_MultiToolWaitingForDischargeQTE.BP_MultiToolWaitingForDischargeQTE_C"))
          (if (Utilities|IsValid _returnvalue_5)
            (Default|UpdateSubBatteryFillAmount _returnvalue_5 _returnvalue_3))))
      ;[0.001 0 1 0.5] Check If This Is Game Over
      (if (== (Variables|Default|GetNumberOfTimeTheCargoHasRespawned) (Variables|Default|GetNumberOfRespawnBeforeExploding))
        (CallFunction|GameOver)))))

(fn GameOver
  (bind _returnvalue (Game|GetPlayerController 0))
  (bind _returnvalue_2 (UserInterface|CreateWidget "/Game/Script/UI/WBP_LooseCanvas.WBP_LooseCanvas_C"))
  (UserInterface|Viewport|AddtoViewport _returnvalue_2 0)
  (Variables|/Script/Engine.PlayerController|SetbShowMouseCursor _returnvalue true)
  (Input|SetInputModeUIOnly _returnvalue _returnvalue_2 "DoNotLock" false))

(fn ResetBatteriesCharge
  (Variables|MainBatteryRotation|SetMainBatteryRotationSpeed (Variables|Default|GetInitialMainBatteryRotationSpeed))
  (Variables|Default|SetNumberOfTimeTheCargoHasRespawned 0)
  ;[0 1 0 0.5] Reset Sub Battery Fill Amount For BP_FirstPersonCharacter And BP_MultiToolWaitingForQTEDischarge
  (Utilities|FlowControl|Sequence
    (:then_0
      (bind _returnvalue (Actor|GetActorOfClass "/Game/FirstPerson/Blueprints/BP_FirstPersonCharacter.BP_FirstPersonCharacter_C"))
      (Default|UpdateSubBatteryFillAmount _returnvalue 0.0))
    (:then_1
      (bind _returnvalue_2 (Actor|GetActorOfClass "/Game/Script/MultiTools/BP_MultiToolWaitingForDischargeQTE.BP_MultiToolWaitingForDischargeQTE_C"))
      (if (Utilities|IsValid _returnvalue_2)
        (Default|UpdateSubBatteryFillAmount _returnvalue_2 0.0)))))