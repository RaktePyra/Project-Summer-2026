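; First-person multitool weapon component that attaches to the character's grip socket, adds weapon input and fires hook and rope projectiles.
; Shoot launches a hook or recalls it once, re-arming after a cooldown triggered by the hook's dispatcher.
; StickySplash cycles through firing two rope anchors joined by a runtime cable, then clearing them.
; Tick updates cable length, and two attached anchors spawn a stretched collision box between them, with a debug trace.
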(event Custom|OnObjectHookedOrIsReturningDispatcher_Event
  (Utilities|FlowControl|Delay (Variables|Default|GetHookCooldown))
  (Variables|Default|SetHasHookBeenLaunched false)
  (Development|PrintString "Hook Cooldown finished")
  (Utilities|FlowControl|DoOnce false) ; enters at Reset
)

(event Custom|OnRopeAttached
  (params (Hit%20Scene%20Component :type Scene%20Component%20Object%20Reference) (Hit%20Location :type Vector))
  (bind _ropeanchorbptable (Variables|Default|GetRopeAnchorBPTable))
  (bind _numberofropeanchored (Variables|Default|GetNumberOfRopeAnchored))
  (Math|Integer|IncrementInt _numberofropeanchored
    (:%20%20
      (switch int _numberofropeanchored
        (:2
          (bind _rope_anchor_world_position (Default|GetRopeAnchorWorldPosition (Utilities|Array|Get(acopy) _ropeanchorbptable)))
          (bind _rope_anchor_world_position_2 (Default|GetRopeAnchorWorldPosition (Utilities|Array|Get(acopy) _ropeanchorbptable 1)))
          (Collision|BoxTraceByChannel (Transformation|GetWorldLocation (Variables|Default|GetCable)) (+ _rope_anchor_world_position_2 "") (/ (Math|Vector|MakeVector (Math|Vector|VectorLength (/ (- (+ _rope_anchor_world_position_2 "") _rope_anchor_world_position) 2.0)) (Variables|Default|GetRope%20Collision%20Box%20Extent%20) 1e+01) 2.0) (Math|Conversions|RotationFromXVector (Math|Vector|Normalize (- (+ _rope_anchor_world_position_2 "") _rope_anchor_world_position))) "TraceTypeQuery1" false 0 "Persistent" true "(R=0.000000,G=0.236701,B=1.000000,A=1.000000)")
          (bind _returnvalue (Game|SpawnActorfromClass "/Game/Script/MultiToolB/BP_RopeBoxCollision.BP_RopeBoxCollision_C" (Math|Transform|MakeTransform (+ (/ (- (+ _rope_anchor_world_position_2 "") _rope_anchor_world_position) 2.0) _rope_anchor_world_position) (Math|Conversions|RotationFromXVector (Math|Vector|Normalize (- (+ _rope_anchor_world_position_2 "") _rope_anchor_world_position))) "1.000000,1.000000,1.000000") "Undefined" "MultiplyWithRoot" 0 0))
          (bind _output_get (Variables|Default|SetRopeCollisionBP _returnvalue))
          (Default|ChangeBoxSize _output_get (Math|Vector|VectorLength (/ (- (+ _rope_anchor_world_position_2 "") _rope_anchor_world_position) 2.0)) (Variables|Default|GetRope%20Collision%20Box%20Extent%20) 1e+01)
          (Development|PrintString "Hello"))))))

(event Input|EnhancedActionEvents|EnhancedInputActionIA_Shoot
  (params (ActionValue :type Boolean) (ElapsedSeconds :type Float%20%28double-precision%29) (TriggeredSeconds :type Float%20%28double-precision%29) (InputAction :type Input%20Action%20Object%20Reference :default "/Game/FirstPerson/Input/Actions/IA_Shoot.IA_Shoot"))
  (if (not (Variables|Default|GetHasHookBeenLaunched))
    (Variables|Default|SetHasHookBeenLaunched true)
    (bind _returnvalue (Game|SpawnActorfromClass "/Game/Script/MultiToolB/BP_HookProjectile.BP_HookProjectile_C" (Math|Transform|MakeTransform (+ (Transformation|GetSocketLocation "Ammo") "0.000000,0.000000,-20.000000") (Camera|GetCameraRotation (Game|GetPlayerCameraManager 0))) "Undefined" "MultiplyWithRoot" 0 (Variables|Default|GetHook%20Max%20Distance) (Components|GetOwner) (Variables|Default|GetHook%20Intensity) 0))
    (bind _output_get (Variables|Default|SetLaunchedHook _returnvalue))
    (EventDispatchers|AssignOnObjectHookedorIsReturningDispatcher _output_get (delegate Custom|OnObjectHookedOrIsReturningDispatcher_Event))
    (else
      (Utilities|FlowControl|DoOnce false
        (:Completed
          (Default|RecallHookProjectile (Variables|Default|GetLaunchedHook)))))))

(event Input|EnhancedActionEvents|EnhancedInputActionIA_StickySplash
  (params (ActionValue :type Boolean) (ElapsedSeconds :type Float%20%28double-precision%29) (TriggeredSeconds :type Float%20%28double-precision%29) (InputAction :type Input%20Action%20Object%20Reference :default "/Game/FirstPerson/Input/Actions/IA_StickySplash.IA_StickySplash"))
  (bind _ropecollisionbp (Variables|Default|GetRopeCollisionBP))
  (bind _cable (Variables|Default|GetCable))
  (switch int (Variables|Default|GetRopeStateIndex)
    (:Default
      (Variables|Default|SetRopeStateIndex 0))
    (:0
      (bind _returnvalue (Game|SpawnActorfromClass "/Game/Script/MultiToolB/BP_RopeProjectile.BP_RopeProjectile_C" (Math|Transform|MakeTransform (+ (Transformation|GetSocketLocation "Ammo") "0.000000,0.000000,-20.000000") (Camera|GetCameraRotation (Game|GetPlayerCameraManager 0))) "Undefined" "MultiplyWithRoot" 0 self 0))
      (Utilities|Array|Add (Variables|Default|GetRopeAnchorBPTable) _returnvalue)
      (Math|Integer|IncrementInt (Variables|Default|GetRopeStateIndex)
        (:%20%20
          (Components|Activation|Activate _cable false)
          (Rendering|ToggleVisibility _cable false)
          (Transformation|AttachComponentToComponent (Variables|Default|GetCable) (Variables|/Game/Script/MultiToolB/BP_RopeProjectile.BP_RopeProjectile_C|GetRopeAnchor _returnvalue) "None" "KeepWorld" "KeepWorld" "KeepWorld" true)
          (Transformation|SetRelativeLocation (Variables|Default|GetCable) "0, 0, 0" false false)
          (Class|CableComponent|SetAttachEndto (Variables|Default|GetCable) (Variables|Default|GetOwnerObject) "None" "None"))))
    (:1
      (bind _returnvalue_2 (Game|SpawnActorfromClass "/Game/Script/MultiToolB/BP_RopeProjectile.BP_RopeProjectile_C" (Math|Transform|MakeTransform (+ (Transformation|GetSocketLocation "Ammo") "0.000000,0.000000,-20.000000") (Camera|GetCameraRotation (Game|GetPlayerCameraManager 0))) "Undefined" "MultiplyWithRoot" 0 self 0))
      (Utilities|Array|Add (Variables|Default|GetRopeAnchorBPTable) _returnvalue_2)
      (Math|Integer|IncrementInt (Variables|Default|GetRopeStateIndex)
        (:%20%20
          (Class|CableComponent|SetAttachEndto (Variables|Default|GetCable) _returnvalue_2 "RopeAnchor" "None")
          (Variables|/Script/CableComponent.CableComponent|SetEndLocation (Variables|Default|GetCable) "0, 0, 0"))))
    (:2
      (for _array_element (Variables|Default|GetRopeAnchorBPTable)
        (Utilities|IsValid _array_element
          (:Is%20Valid
            (Actor|DestroyActor _array_element))))
      (Variables|Default|SetRopeStateIndex 0)
      (Transformation|DetachFromComponent (Variables|Default|GetCable) "KeepWorld" "KeepWorld" "KeepWorld" true)
      (Transformation|SetWorldLocation (Variables|Default|GetCable) (Transformation|GetSocketLocation (Variables|/Script/Engine.Actor|GetRootComponent (Variables|Default|GetOwnerObject)) "Ammo") false false)
      (Rendering|ToggleVisibility (Variables|Default|GetCable) false)
      (Variables|Default|SetNumberOfRopeAnchored 0)
      (Utilities|Array|Clear (Variables|Default|GetRopeAnchorBPTable))
      (Utilities|IsValid _ropecollisionbp
        (:Is%20Valid
          (Actor|DestroyActor _ropecollisionbp))))))

(event EventBeginPlay
  (Utilities|FlowControl|Sequence
    (:then_0
      (bind _output_get (Variables|Default|SetOwnerObject (Components|GetOwner)))
      (bind _asbp_first_person_character (Utilities|Casting|CastToBP_FirstPersonCharacter _output_get))
      (Variables|Default|SetAs%20BP%20First%20Person%20Character _asbp_first_person_character)
      (Transformation|AttachComponentToComponent (Variables|/Game/FirstPerson/Blueprints/BP_FirstPersonCharacter.BP_FirstPersonCharacter_C|GetFirstPersonMesh _asbp_first_person_character) "GripPoint" "SnapToTarget" "SnapToTarget" "SnapToTarget" true)
      (bind _asplayer_controller (Utilities|Casting|CastToPlayerController (Pawn|GetController (Variables|Default|GetAs%20BP%20First%20Person%20Character))))
      (Utilities|IsValid (PlayerController|LocalPlayerSubsystems|GetEnhancedInputLocalPlayerSubsystem _asplayer_controller)
        (:Is%20Valid
          (Input|AddMappingContext (PlayerController|LocalPlayerSubsystems|GetEnhancedInputLocalPlayerSubsystem _asplayer_controller) "/Game/FirstPerson/Input/IMC_Weapons.IMC_Weapons" 0 "(bIgnoreAllPressedKeysUntilRelease=True,bForceImmediately=False,bNotifyUserSettings=False)")
          (bind _asfirst_person_anim_bp (Utilities|Casting|CastToFirstPerson_AnimBP (Components|SkeletalMesh|GetAnimInstance (Variables|/Game/FirstPerson/Blueprints/BP_FirstPersonCharacter.BP_FirstPersonCharacter_C|GetFirstPersonMesh (Variables|Default|GetAs%20BP%20First%20Person%20Character)))))
          (Variables|/Game/FirstPersonArms/Animations/FirstPerson_AnimBP.FirstPerson_AnimBP_C|SetHasRifle _asfirst_person_anim_bp true))))
    (:then_1
      (bind _returnvalue (Game|AddComponentbyClass (Variables|Default|GetOwnerObject) "/Script/CableComponent.CableComponent" false))
      (Variables|Default|SetCable _returnvalue)
      (Transformation|AttachComponentToComponent (Variables|Default|GetCable) (Variables|/Script/Engine.Actor|GetRootComponent (Variables|Default|GetOwnerObject)) "None" "KeepRelative" "KeepRelative" "KeepRelative" true))
    (:then_2
      (EventDispatchers|BindEventtoOnRopeAttachedDispatcher (delegate Custom|OnRopeAttached)))
    (:then_3
      (Components|Activation|Deactivate (Variables|Default|GetCable))
      (Rendering|ToggleVisibility (Variables|Default|GetCable) false))))

(event EventTick
  (params (DeltaSeconds :type Float%20%28single-precision%29))
  (if (> (Variables|Default|GetRopeStateIndex) 0)
    (Variables|/Script/CableComponent.CableComponent|SetCableLength (Variables|Default|GetCable) (Math|Vector|VectorLength (- (Transformation|GetWorldLocation (Class|CableComponent|GetAttachedComponent (Variables|Default|GetCable))) (+ (Variables|/Script/CableComponent.CableComponent|GetEndLocation (Variables|Default|GetCable)) (Transformation|GetActorLocation (Class|CableComponent|GetAttachedActor (Variables|Default|GetCable)))))))))