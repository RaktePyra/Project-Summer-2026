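; BP_MovingObject is a level feature actor that moves its MovingObject component along a Spline when play begins.
; On BeginPlay it caches the object's world rotation and scale, then plays the MoveAlongSpline timeline from the start.
; Each update maps the timeline alpha to a distance along the spline and applies only that location, keeping the cached rotation and scale.
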(event EventBeginPlay
  (Variables|Default|SetMovingObjectRotation (Transformation|GetWorldRotation (Variables|Default|GetMovingObject)))
  (Variables|Default|SetMovingObjectScale (Transformation|GetWorldScale (Variables|Default|GetMovingObject)))
  (bind _alpha (Timeline|Move%20Along%20Spline PlayFromStart)
    (:Update
      (Transformation|SetWorldTransform (Variables|Default|GetMovingObject) (Math|Transform|MakeTransform (.location (Spline|GetTransformatDistanceAlongSpline (Variables|Default|GetSpline) (* _alpha (Spline|GetSplineLength (Variables|Default|GetSpline))) "World" false)) (Variables|Default|GetMovingObjectRotation) (Variables|Default|GetMovingObjectScale)) false false))))

(fn ConstructionScript)