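; BP_Checkpoint is a checkpoint actor that updates where the cargo respawns when the cargo reaches it.
; On begin play it caches the level's BP_Cargo, and when that actor overlaps the trigger box it copies the RespawnCargo component's transform into BP_DeliveryZone's respawn location and rotation.
; The same overlap turns on four lights.
; Each tick, the checkpoint text rotates to face the player camera.
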(event OnComponentBeginOverlap(CheckPointTriggerBox)
  (params (OverlappedComponent :type Primitive%20Component%20Object%20Reference) (OtherActor :type Actor%20Object%20Reference) (OtherComp :type Primitive%20Component%20Object%20Reference) (OtherBodyIndex :type Integer) (bFromSweep :type Boolean) (SweepResult :type Hit%20Result%20Structure%20%28by%20ref%29))
  (bind _respawncargo (Variables|Default|GetRespawnCargo))
  ;[1 0 0 0.5] Set Cargo Respawn Position And Rotation
  (if (== OtherActor (Variables|Default|GetCargo))
    (bind _returnvalue (Actor|GetActorOfClass "/Game/Script/Cargo/BP_DeliveryZone.BP_DeliveryZone_C"))
    (Variables|/Game/Script/Cargo/BP_DeliveryZone.BP_DeliveryZone_C|SetRespawnLocation _returnvalue (Transformation|GetWorldLocation _respawncargo))
    (Variables|/Game/Script/Cargo/BP_DeliveryZone.BP_DeliveryZone_C|SetRespawnRotation _returnvalue (Transformation|GetWorldRotation _respawncargo))
    (Rendering|SetVisibility (Variables|Default|GetLight) true false)))

(event EventTick
  (params (DeltaSeconds :type Float%20%28single-precision%29))
  ;[0 0.5 0.5 0.5] Rotate TextCheckPoint
  (Transformation|SetWorldRotation (Variables|Default|GetTextCheckpoint) (Math|Rotator|FindLookatRotation (Transformation|GetWorldLocation (Variables|Default|GetTextCheckpoint)) (Camera|GetCameraLocation (Game|GetPlayerCameraManager 0))) false false))

(event EventBeginPlay
  ;[0.5 0.5 0 0.5] Set Cargo Variable
  (bind _returnvalue (Actor|GetActorOfClass "/Game/Script/Cargo/BP_Cargo.BP_Cargo_C"))
  (Variables|Default|SetCargo _returnvalue))

(fn ConstructionScript)