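; BP_Cargo is the physics cargo the player delivers to win the game.
; On BeginPlay it stores the cargo's starting transform and shows the hotkeys widget.
; When DeliveryZone reports an overlap with this actor itself, it shows the win screen and ignores player move input.
; RespawnCargo, not called within this Blueprint, restores the saved transform and zeroes linear and angular velocity.
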(event OnComponentBeginOverlap(DeliveryZone)
  (params (OverlappedComponent :type Primitive%20Component%20Object%20Reference) (OtherActor :type Actor%20Object%20Reference) (OtherComp :type Primitive%20Component%20Object%20Reference) (OtherBodyIndex :type Integer) (bFromSweep :type Boolean) (SweepResult :type Hit%20Result%20Structure%20%28by%20ref%29))
  ;[0 0.998 0 0.5] Win Condition
  (if (== OtherActor self)
    (bind _returnvalue (UserInterface|CreateWidget "/Game/Script/UI/WBP_WinCanvas.WBP_WinCanvas_C"))
    (UserInterface|Viewport|AddtoViewport _returnvalue 0)
    (Input|SetIgnoreMoveInput (Game|GetPlayerController 0) true)))

(event EventBeginPlay
  (Utilities|FlowControl|Sequence
    (:then_0
      ;[0 0 1 0.5] Set Respawn Location and Rotation Variables
      (Variables|Default|SetRespawnLocation (Transformation|GetWorldLocation (Variables|Default|GetCargo)))
      (Variables|Default|SetRespawnRotation (Transformation|GetWorldRotation (Variables|Default|GetCargo))))
    (:then_1
      ;[1 0 0 0.5] Add The Hot Keys WBP To Screen
      (bind _returnvalue (UserInterface|CreateWidget "/Game/Script/UI/WBP_HotKeys.WBP_HotKeys_C"))
      (UserInterface|Viewport|AddtoPlayerScreen _returnvalue))))

(fn ConstructionScript)

(fn RespawnCargo
  (Transformation|SetWorldLocationAndRotation (Variables|Default|GetCargo) (Variables|Default|GetRespawnLocation) (Variables|Default|GetRespawnRotation) false false)
  (Physics|SetPhysicsLinearVelocity (Variables|Default|GetCargo) "0, 0, 0" false "None")
  (Class|PrimitiveComponent|SetPhysicsAngularVelocityinDegrees (Variables|Default|GetCargo) "0, 0, 0" false "None"))